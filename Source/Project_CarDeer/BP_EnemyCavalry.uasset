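; BP_EnemyCavalry is an enemy chess piece that moves two grid steps when ShouldAction fires.
; Action chains two FindNextLocation calls, retrying in a bounded loop for a free tile at Manhattan distance two.
; It then transfers tile occupancy and sets Destination above that tile, even if every retry failed.
; BeginPlay caches the player piece; an unconnected recursive version of the move remains in Action.
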(event EventBeginPlay
  (bind _outactors (Actor|GetAllActorsOfClass "/Game/Blueprints/Player/BP_PlayerChess.BP_PlayerChess_C"))
  (Variables|Default|SetTargetPlayerChess (Utilities|Array|Get(acopy) _outactors)))

(event Collision|EventActorBeginOverlap
  (params (OtherActor :type Actor%20Object%20Reference)))

(event EventTick
  (params (DeltaSeconds :type Float%20%28single-precision%29)))

(event EventShouldAction
  (CallFunction|Action))

(fn ConstructionScript)

(fn Action
  (Utilities|FlowControl|ForLoopwithBreak 0 40 :!label _label
    (:LoopBody
      (bind (_targetrow _targetcolumn) (Class|EnemyPawn|FindNextLocation (Variables|Default|GetSelfIndexX) (Variables|Default|GetSelfIndexY)))
      (bind (_targetrow_2 _targetcolumn_2) (Class|EnemyPawn|FindNextLocation _targetrow _targetcolumn))
      (bind _outactors (Actor|GetAllActorsOfClass "/Game/Blueprints/BlockMap/BP_MapArranger.BP_MapArranger_C"))
      (bind _returnvalue (Class|MapArranger|GetMapUnitInstance (Utilities|Array|Get(acopy) _outactors) _targetrow_2 _targetcolumn_2))
      (if (== (+ (Math|Integer|Absolute(Integer) (- _targetrow_2 (Variables|Default|GetSelfIndexX))) (Math|Integer|Absolute(Integer) (- _targetcolumn_2 (Variables|Default|GetSelfIndexY)))) 2)
        (if (not (Variables|/Script/Project_CarDeer.MapUnit|GetbEnemySteppingOn _returnvalue))
          (goto _label Break))))
    (:Completed
      (Variables|/Script/Project_CarDeer.MapUnit|SetbEnemySteppingOn _returnvalue true)
      (Variables|/Script/Project_CarDeer.MapUnit|SetActorSteppedOn _returnvalue 0)
      (Variables|/Script/Project_CarDeer.MapUnit|SetbEnemySteppingOn (Variables|Default|GetSteppedOnUnit) false)
      (Variables|Default|SetDestination (+ (Transformation|GetActorLocation _returnvalue) "0.000000,0.000000,100.000000"))
      (return true))))