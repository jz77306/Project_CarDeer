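; BP_RoundCenter sets up a grid-based chess and card match and starts rounds through the player controller.
; On BeginPlay it binds the map and enemy arranger, spawns the player chess on a random tile, then two enemies.
; Enemies are randomly soldier or cavalry, placed by bounded random retries for a free tile, and registered with the arranger.
; It then deals four cards from the pile with short delays before calling AnotherRound.
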(event Custom|AnotherRound
  (bind _asbp_car_deer_player_controller (Utilities|Casting|CastToBP_CarDeerPlayerController (Game|GetPlayerController 0)))
  (Default|AnotherRound _asbp_car_deer_player_controller))

(event EventBeginPlay
  (Utilities|BindMap&EnemyArranger)
  (bind _palyerchessspawned (CallFunction|SpawnPlayerChess))
  (Variables|Default|SetPalyer%20Chess%20Spawned _palyerchessspawned)
  (CallFunction|SpawnEnemy 2)
  (bind _outactors (Actor|GetAllActorsOfClass "/Game/Blueprints/Player/BP_CardPile.BP_CardPile_C"))
  (Variables|Default|SetTarget%20Card%20Pile (Utilities|Array|Get(acopy) _outactors))
  (Utilities|NewMacro)
  (Utilities|NewMacro)
  (Utilities|NewMacro)
  (Utilities|NewMacro)
  (CallFunction|AnotherRound))

(fn ConstructionScript)

(fn FindEnemySpawnLocation
  (bind _returnvalue (Math|Random|RandomInteger 5))
  (bind _returnvalue_2 (Math|Random|RandomInteger 5))
  (bind _outactors (Actor|GetAllActorsOfClass "/Game/Blueprints/Player/BP_PlayerChess.BP_PlayerChess_C"))
  (Utilities|FlowControl|ForLoopwithBreak 0 40 :!label _label
    (:LoopBody
      (bind _returnvalue_3 (Class|MapArranger|GetMapUnitInstance (Variables|Default|GetBlockMap) _returnvalue_2 _returnvalue))
      (if (>= (+ (Math|Integer|Absolute(Integer) (- _returnvalue_2 (Variables|/Script/Project_CarDeer.MapUnit|GetRowIndex (Variables|/Script/Project_CarDeer.PlayerChess|GetSteppedOnUnit (Utilities|Array|Get(acopy) _outactors))))) (Math|Integer|Absolute(Integer) (- _returnvalue (Variables|/Script/Project_CarDeer.MapUnit|GetColumnIndex (Variables|/Script/Project_CarDeer.PlayerChess|GetSteppedOnUnit (Utilities|Array|Get(acopy) _outactors)))))) 3)
        (if (not (Variables|/Script/Project_CarDeer.MapUnit|GetbPlayerSteppingOn _returnvalue_3))
          (if (not (Variables|/Script/Project_CarDeer.MapUnit|GetbEnemySteppingOn _returnvalue_3))
            (goto _label Break)))))
    (:Completed
      (return _returnvalue_3 (Variables|/Script/Project_CarDeer.MapUnit|GetRowIndex _returnvalue_3) (Variables|/Script/Project_CarDeer.MapUnit|GetColumnIndex _returnvalue_3)))))

(fn SpawnEnemy
  (params (NumOfEnemy :type Integer))
  (bind _enemyarranger (Variables|Default|GetEnemyArranger))
  (bind _palyer_chess_spawned (Variables|Default|GetPalyer%20Chess%20Spawned))
  (bind _possessenemyarray (Variables|/Game/Blueprints/Enemy/BP_EnemyArranger.BP_EnemyArranger_C|GetPossessEnemyArray _enemyarranger))
  (for _index (range 1 NumOfEnemy)
    (bind (_mapblock _row_index _column_index) (CallFunction|FindEnemySpawnLocation))
    (if (>= (Math|Random|RandomInteger 3) 2)
      ;[1 1 1] 生成+初始化变量
      (bind _returnvalue (Game|SpawnActorfromClass "/Game/Blueprints/Enemy/BP_EnemyCavalry.BP_EnemyCavalry_C" (Math|Transform|MakeTransform (+ (Transformation|GetActorLocation _mapblock) "0.000000,0.000000,100.000000") "0, 0, 0" "1.000000,1.000000,1.000000") "AdjustIfPossibleButAlwaysSpawn" "MultiplyWithRoot" 0 0))
      (Class|EnemyPawn|InitIndex _returnvalue _row_index _column_index)
      (Utilities|Array|Add _possessenemyarray _returnvalue)
      (Utilities|FlowControl|Sequence
        (:then_0
          (Variables|/Script/Project_CarDeer.EnemyPawn|SetSteppedOnUnit _returnvalue _mapblock))
        (:then_1
          (Variables|/Script/Project_CarDeer.EnemyPawn|SetTargetPlayerChess _returnvalue _palyer_chess_spawned))
        (:then_2
          (Variables|/Script/Project_CarDeer.MapUnit|SetbEnemySteppingOn _mapblock true))
        (:then_3
          (Variables|/Script/Project_CarDeer.MapUnit|SetActorSteppedOn _mapblock _returnvalue)))
      (else
        (bind _returnvalue_2 (Game|SpawnActorfromClass "/Game/Blueprints/Enemy/BP_EnemySoldier.BP_EnemySoldier_C" (Math|Transform|MakeTransform (+ (Transformation|GetActorLocation _mapblock) "0.000000,0.000000,100.000000") "0, 0, 0" "1.000000,1.000000,1.000000") "AdjustIfPossibleButAlwaysSpawn" "MultiplyWithRoot" 0 0))
        (Class|EnemyPawn|InitIndex _returnvalue_2 _row_index _column_index)
        (Utilities|Array|Add _possessenemyarray _returnvalue_2)
        (Utilities|FlowControl|Sequence
          (:then_0
            (Variables|/Script/Project_CarDeer.EnemyPawn|SetSteppedOnUnit _returnvalue_2 _mapblock))
          (:then_1
            (Variables|/Script/Project_CarDeer.EnemyPawn|SetTargetPlayerChess _returnvalue_2 _palyer_chess_spawned))
          (:then_2
            (Variables|/Script/Project_CarDeer.MapUnit|SetbEnemySteppingOn _mapblock true))
          (:then_3
            (Variables|/Script/Project_CarDeer.MapUnit|SetActorSteppedOn _mapblock _returnvalue_2)))))))

(fn SpawnPlayerChess
  (bind _returnvalue (Class|MapArranger|GetMapUnitInstance (Variables|Default|GetBlockMap) (Math|Random|RandomInteger 5) (Math|Random|RandomInteger 5)))
  (bind _returnvalue_2 (Game|SpawnActorfromClass "/Game/Blueprints/Player/BP_PlayerChess.BP_PlayerChess_C" (Math|Transform|MakeTransform (Math|Vector|MakeVector (.x (Transformation|GetActorLocation _returnvalue)) (.y (Transformation|GetActorLocation _returnvalue)) (+ (.z (Transformation|GetActorLocation _returnvalue)) 1e+02)) "0, 0, 0" "1.000000,1.000000,1.000000") "AdjustIfPossibleButAlwaysSpawn" "MultiplyWithRoot" 0 0))
  (Utilities|FlowControl|Sequence
    (:then_0
      (Variables|/Script/Project_CarDeer.MapUnit|SetbPlayerSteppingOn _returnvalue true))
    (:then_1
      (Variables|/Script/Project_CarDeer.MapUnit|SetActorSteppedOn _returnvalue _returnvalue_2))
    (:then_2
      (Variables|/Script/Project_CarDeer.PlayerChess|SetSteppedOnUnit _returnvalue_2 _returnvalue)
      (return _returnvalue_2))))

(fn DrawCard
  (return 0))