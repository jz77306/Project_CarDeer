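; BP_Card_Move_02 is a movement card that, when launched, gathers target map units around the tile the player's chess piece stands on.
; A two-pass loop flips the sign of Step, adding attack targets on both sides along the row index and move targets on both sides along the column index.
; It then passes TargetMapUnits to the player pawn's MoveCard and destroys the card.
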(event EventBeginPlay
  (|CallParentFunction))

(event Collision|EventActorBeginOverlap
  (params (OtherActor :type Actor%20Object%20Reference)))

(event EventTick
  (params (DeltaSeconds :type Float%20%28single-precision%29)))

(event EventCardLaunchEffect
  (bind _playerchess (Variables|Default|GetPlayerChess))
  (bind _steppedonunit (Variables|/Script/Project_CarDeer.PlayerChess|GetSteppedOnUnit _playerchess))
  (Variables|Default|SetRow (Class|MapUnit|GetRowIndex _steppedonunit))
  (Variables|Default|SetColumn (Class|MapUnit|GetColumnIndex _steppedonunit))
  (for _index (range 0 1)
    (CallFunction|AddAttackTargetMapUnits (+ (Variables|Default|GetRow) (Variables|Default|GetStep)) (Variables|Default|GetColumn))
    (CallFunction|AddMoveTargetMapUnits (Variables|Default|GetRow) (+ (Variables|Default|GetColumn) (Variables|Default|GetStep)))
    (Variables|Default|SetStep (* (Variables|Default|GetStep) -1)))
  (Default|MoveCard (Variables|Default|GetPlayerPawn) (Variables|Default|GetTargetMapUnits))
  (CallFunction|DestroyCard))

(fn ConstructionScript)