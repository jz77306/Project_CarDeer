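; BP_AnotherCard_MagicSquare is a player card that attacks map units lying on intersecting rows and columns.
; On launch it asks MapArranger for row/column intersections, gathers every unit in those rows and columns without duplicates, and passes them to the player pawn's AttackCard.
; With no intersections, it has BP_CardPile draw the same card class back into the hand.
; The card then destroys itself.
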(event EventBeginPlay
  (|CallParentFunction))

(event EventCardLaunchEffect
  (bind _returnvalue (Class|MapArranger|GetRowColumnIntersection (Variables|Default|GetMapArranger)))
  (if (Utilities|Array|IsNotEmpty _returnvalue)
    (for _array_element _returnvalue
      (bind _returnvalue_2 (Class|MapArranger|GetTotalRowColUnitInstance (Variables|Default|GetMapArranger) (Variables|/Script/Project_CarDeer.MapUnit|GetRowIndex _array_element) (Variables|/Script/Project_CarDeer.MapUnit|GetColumnIndex _array_element)))
      (for _array_element_2 _returnvalue_2
        (bind _asbp_map_unit (Utilities|Casting|CastToBP_MapUnit _array_element_2))
        (if (== (Utilities|Array|FindItem (Variables|Default|GetTargetMapUnits) _asbp_map_unit) -1)
          (Utilities|Array|Add (Variables|Default|GetTargetMapUnits) _asbp_map_unit))))
    (Default|AttackCard (Variables|Default|GetPlayerPawn) (Variables|Default|GetTargetMapUnits) 1 4)
    (else
      (bind _outactors (Actor|GetAllActorsOfClass "/Game/Blueprints/Player/BP_CardPile.BP_CardPile_C"))
      (bind _newcard (Class|BPIGameBasic|DrawCard(Message) (Utilities|Array|Get(acopy) _outactors) "BP_AnotherCard_MagicSquare_C"))
      (Class|BPIGameBasic|AddCardtoHand(Message) (Variables|Default|GetPlayerPawn) _newcard)))
  (CallFunction|DestroyCard))

(fn ConstructionScript
  (|CallParentFunction))