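; BP_Card_Attack is a player attack card that works out which map tiles the player's chess piece can target.
; ObtainAttackRange reads the row and column of the piece's tile, then scans every BP_MapUnit in the level.
; Units at Manhattan distance one or two become targets, forming a diamond that excludes the piece's own tile.
; The target list is passed to PlayerPawn's AttackCard along with DigitChange and AttackMode.
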(event Custom|Obtain%20Attack%20Range
  (params (DigitChange :type Integer) (AttackMode :type Integer))
  (bind _playerchess (Variables|Default|GetPlayerChess))
  (bind _steppedonunit (Variables|/Script/Project_CarDeer.PlayerChess|GetSteppedOnUnit _playerchess))
  (Variables|Default|SetRow (Class|MapUnit|GetRowIndex _steppedonunit))
  (Variables|Default|SetColumn (Class|MapUnit|GetColumnIndex _steppedonunit))
  (bind _outactors (Actor|GetAllActorsOfClass "/Game/Blueprints/BlockMap/BP_MapUnit.BP_MapUnit_C"))
  (for _array_element _outactors
    (if (== (+ (Math|Integer|Absolute(Integer) (- (Variables|Default|GetRow) (Class|MapUnit|GetRowIndex _array_element))) (Math|Integer|Absolute(Integer) (- (Variables|Default|GetColumn) (Class|MapUnit|GetColumnIndex _array_element)))) 2)
      (CallFunction|AddTargetMapUnits (Class|MapUnit|GetRowIndex _array_element) (Class|MapUnit|GetColumnIndex _array_element) :!label _label)
      (elif (== (+ (Math|Integer|Absolute(Integer) (- (Variables|Default|GetRow) (Class|MapUnit|GetRowIndex _array_element))) (Math|Integer|Absolute(Integer) (- (Variables|Default|GetColumn) (Class|MapUnit|GetColumnIndex _array_element)))) 1)
        (goto _label))))
  (Default|AttackCard (Variables|Default|GetPlayerPawn) (Variables|Default|GetTargetMapUnits) DigitChange AttackMode))

(event EventBeginPlay
  (|CallParentFunction))

(event Collision|EventActorBeginOverlap
  (params (OtherActor :type Actor%20Object%20Reference)))

(event EventTick
  (params (DeltaSeconds :type Float%20%28single-precision%29)))

(fn ConstructionScript)