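; BP_PlayerChess is the player's chess piece, which moves between board units and can be raised or lowered.
; Move sets Destination above the target unit and transfers the stepped-on state and references; the travel toward Destination happens outside these graphs.
; Rise and reset events shift Destination vertically.
; NewFunction prints debug text, then plays a floating sequence at a rate-derived speed or reverses it.
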(event EventBeginPlay)

(event Collision|EventActorBeginOverlap
  (params (OtherActor :type Actor%20Object%20Reference)))

(event EventTick
  (params (DeltaSeconds :type Float%20%28single-precision%29)))

(event EventPlayerMove
  (params (TargetLocation :type Map%20Unit%20Object%20Reference))
  (CallFunction|Move TargetLocation))

(event EventChessRise
  (params (AnimationSecond :type Float%20%28double-precision%29))
  ;[1 1 1] 棋子的上升下降
  (Variables|Default|SetDestination (+ (Variables|Default|GetDestination) "0.000000,0.000000,100.000000")))

(event EventChessHeightReset
  (params (AnimationSecond :type Float%20%28double-precision%29))
  ;[1 1 1] 棋子的上升下降
  (Variables|Default|SetDestination (+ (Variables|Default|GetDestination) "0.000000,0.000000,-100.000000")))

(fn ConstructionScript)

(fn NewFunction
  (params (Enable :type Boolean) (Rate :type Float%20%28double-precision%29))
  (bind _floatingsequence (Variables|Default|GetFloatingSequence))
  (bind _sequenceplayer (Variables|/Script/ActorSequence.ActorSequenceComponent|GetSequencePlayer _floatingsequence))
  (Utilities|FlowControl|Sequence
    (:then_0
      (Development|PrintText (Utilities|Text|FormatText "{Name} Floating 
Reverse {bool}" (Utilities|GetDisplayName self))))
    (:then_1
      (Variables|Default|SetAnimationSecond (/ 1.0 (Math|Float|Max(Float) 0.0 0.001)))
      (if Enable
        (Components|Timeline|SetPlayRate _sequenceplayer (Variables|Default|GetAnimationSecond))
        (Sequencer|Player|Play _sequenceplayer :!class /Script/MovieScene.MovieSceneSequencePlayer)
        (else
          (Class|MovieSceneSequencePlayer|PlayReverse _sequenceplayer)))
      (return (Variables|Default|GetAnimationSecond)))))

(fn Move
  (params (TargetLocation :type Map%20Unit%20Object%20Reference))
  (Variables|/Script/Project_CarDeer.MapUnit|SetbPlayerSteppingOn (Variables|Default|GetSteppedOnUnit) false)
  (Variables|Default|SetDestination (+ (Transformation|GetActorLocation TargetLocation) "0.000000,0.000000,100.000000"))
  (Variables|/Script/Project_CarDeer.MapUnit|SetbPlayerSteppingOn TargetLocation true)
  (Variables|Default|SetSteppedOnUnit TargetLocation)
  (Variables|/Script/Project_CarDeer.MapUnit|SetActorSteppedOn TargetLocation self))