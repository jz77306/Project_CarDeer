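; BP_CarDeerPlayerController is the player controller for a turn-based card game, handling card input and round switching.
; Left mouse press draws from a hit card pile and sends the card to the pawn's hand, while release triggers playing a card.
; Space bar activates enemies through BP_EnemyArranger.
; AnotherRound uses a FlipFlop to alternate the player's round, refilling BP_PlayerPawn mana when it begins.
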(event Custom|AnotherRound
  (Utilities|FlowControl|FlipFlop
    (:A
      (Variables|Default|SetIsPlayerRound true)
      (bind _asbp_player_pawn (Utilities|Casting|CastToBP_PlayerPawn (Game|Player|GetPlayerPawn 0)))
      (Variables|/Script/Project_CarDeer.PlayerPawn|SetMana _asbp_player_pawn 4))
    (:B
      (Variables|Default|SetIsPlayerRound false))))

(event EventBeginPlay)

(event EventTick
  (params (DeltaSeconds :type Float%20%28single-precision%29)))

(event Input|MouseEvents|LeftMouseButton
  (params (Key :type Key%20Structure :default "None"))
  (:Pressed
    (Class|ProjectCarDeerPlayerController|LeftMousePress)
    (if (Variables|Default|GetbHitCardPile)
      (if (not (Variables|Default|GetHaveDrawCard))
        (bind _newcard (Class|BPIGameBasic|DrawCard(Message) (Variables|Default|GetTargetCardPile)))
        (Class|BPIGameBasic|AddCardtoHand(Message) (Game|Player|GetPlayerPawn 0) _newcard)
        (Variables|Default|SetbHitCardPile false)
        (Variables|Default|SetHaveDrawCard false))))
  (:Released
    (Class|ProjectCarDeerPlayerController|LeftMouseRelease)
    (if (Variables|Default|GetbCardPlayed)
      (Class|BPIGameBasic|PlayCard(Message) (Game|Player|GetPlayerPawn 0)))))

(event Input|KeyboardEvents|SpaceBar
  (params (Key :type Key%20Structure :default "None"))
  (:Pressed
    (bind _outactors (Actor|GetAllActorsOfClass "/Game/Blueprints/Enemy/BP_EnemyArranger.BP_EnemyArranger_C"))
    (Class|BPIEnemy|ActivateEnemies(Message) (Utilities|Array|Get(acopy) _outactors))))

(fn ConstructionScript)

(fn DrawCard)