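; Player pawn for a card-driven tile-grid tactics game, handling the hand, mana and resolution of move and attack cards.
; Move and attack cards spend mana and raise indicators on target tiles; ReleaseAbility validates the chosen tile, then moves the chess piece or applies damage, tile-number changes and effects.
; Tick arranges the hand and outlines tiles under the cursor by glow mode: single, row, column, neighbours or cross.
; Spending the last mana starts another round.
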(event Custom|Move%20Card
  (params (TargetMapUnits :type Array%20of%20BP%20Map%20Unit%20Object%20References))
  (Utilities|UsingMana)
  (bind _output_get (Variables|Default|SetTarget%20Map%20Units TargetMapUnits))
  (for _array_element _output_get
    (Default|玩家棋子可移动格子指示器（需升起） _array_element true 0.5))
  (Variables|Default|SetCanMove true))

(event Custom|Attack%20Card
  (params (TargetMapUnits :type Array%20of%20BP%20Map%20Unit%20Object%20References) (DigitChange :type Integer) (AttackMode :type Integer))
  (Utilities|UsingMana)
  (Utilities|SetAttackInfo TargetMapUnits DigitChange AttackMode)
  (for _array_element (Variables|Default|GetTarget%20Map%20Units)
    (Default|玩家可攻击格子指示器（需升起） _array_element true 0.5))
  (Variables|Default|SetCanAttack true))

(event EventBeginPlay
  (CameraShakes|StartCameraShake (Game|GetPlayerCameraManager 0) "/Game/Blueprints/CameraShake/BP_CameraShake.BP_CameraShake_C" 1.0 "CameraLocal" "0, 0, 0")
  (Utilities|FlowControl|Delay 0.5)
  (bind _outactors (Actor|GetAllActorsOfClass "/Script/Project_CarDeer.MapArranger"))
  (Variables|Default|SetMapArranger (Utilities|Array|Get(acopy) _outactors))
  (bind _outactors_2 (Actor|GetAllActorsOfClass "/Game/Blueprints/Player/BP_PlayerChess.BP_PlayerChess_C"))
  (Variables|Default|SetPlayerChess (Utilities|Array|Get(acopy) _outactors_2))
  (bind _outactors_3 (Actor|GetAllActorsOfClass "/Game/Blueprints/Miscellaneous/BP_ManaLight.BP_ManaLight_C"))
  (Variables|Default|SetManaLight (Utilities|Array|Get(acopy) _outactors_3))
  (bind _asbp_car_deer_player_controller (Utilities|Casting|CastToBP_CarDeerPlayerController (Game|GetPlayerController 0)))
  (Variables|Default|SetPlayer%20Controller _asbp_car_deer_player_controller))

(event Collision|EventActorBeginOverlap
  (params (OtherActor :type Actor%20Object%20Reference)))

(event EventTick
  (params (DeltaSeconds :type Float%20%28single-precision%29))
  (bind _returnvalue (Game|GetPlayerController 0))
  (bind _glowingmapunits (Variables|Default|GetGlowingMapUnits))
  (bind _hitresult (Game|Player|GetHitResultUnderCursorbyChannel _returnvalue "TraceTypeQuery1" true))
  (bind _hitactor (Collision|BreakHitResult _hitresult))
  ;[1 1 1] 整理手牌
  (Utilities|FlowControl|Sequence
    (:then_0
      (for (_array_element _array_index) (Variables|Default|GetArrCardsInHand)
        (if (not (Variables|/Script/Project_CarDeer.ParentCard|GetbIsSelected _array_element))
          (Variables|/Script/Project_CarDeer.ParentCard|SetPositionInHand _array_element (Utilities|Array|Get(acopy) (Variables|Default|GetArrInHandPosition) _array_index)))))
    (:then_1
      (if (Variables|Default|GetCanGlowMapUnit)
        (if (Utilities|Array|IsEmpty _glowingmapunits)
          _
          (else
            (CallFunction|MakeMapUnitsDark _glowingmapunits)
            (Utilities|Array|Clear (Variables|Default|GetGlowingMapUnits))))
        (bind _asbp_enemy_cavalry (Utilities|Casting|CastToBP_EnemyCavalry _hitactor)
          (:then
            (bind _asbp_map_unit (Utilities|Casting|CastToBP_MapUnit (Variables|/Script/Project_CarDeer.EnemyPawn|GetSteppedOnUnit _asbp_enemy_cavalry)))
            (if (!= (Utilities|Array|FindItem (Variables|Default|GetTarget%20Map%20Units) _asbp_map_unit) -1)
              (CallFunction|MakeMapUnitsGlow _asbp_map_unit)))
          (:CastFailed
            (bind _asbp_enemy_soldier (Utilities|Casting|CastToBP_EnemySoldier _hitactor)
              (:then
                (bind _asbp_map_unit_2 (Utilities|Casting|CastToBP_MapUnit (Variables|/Script/Project_CarDeer.EnemyPawn|GetSteppedOnUnit _asbp_enemy_soldier)))
                (if (!= (Utilities|Array|FindItem (Variables|Default|GetTarget%20Map%20Units) _asbp_map_unit_2) -1)
                  (CallFunction|MakeMapUnitsGlow _asbp_map_unit_2)))
              (:CastFailed
                (bind _asbp_player_chess (Utilities|Casting|CastToBP_PlayerChess _hitactor)
                  (:then
                    (bind _asbp_map_unit_3 (Utilities|Casting|CastToBP_MapUnit (Variables|/Script/Project_CarDeer.PlayerChess|GetSteppedOnUnit _asbp_player_chess)))
                    (if (!= (Utilities|Array|FindItem (Variables|Default|GetTarget%20Map%20Units) _asbp_map_unit_3) -1)
                      (CallFunction|MakeMapUnitsGlow _asbp_map_unit_3)))
                  (:CastFailed
                    (bind _asbp_map_unit_4 (Utilities|Casting|CastToBP_MapUnit _hitactor))
                    (if (!= (Utilities|Array|FindItem (Variables|Default|GetTarget%20Map%20Units) _asbp_map_unit_4) -1)
                      (CallFunction|MakeMapUnitsGlow _asbp_map_unit_4))))))))))))

(event EventAddCardtoHand
  (params (NewCard :type Actor%20Object%20Reference))
  ;[1 1 1] 抽卡
  (bind _asbp_parent_card (Utilities|Casting|CastToBP_ParentCard NewCard))
  (bind _returnvalue (Class|PlayerPawn|AddCard _asbp_parent_card))
  (if _returnvalue
    (Class|BPIGameBasic|BurnCard(Message) NewCard)
    (else
      (bind _returnvalue_2 (Utilities|Array|Add (Variables|Default|GetArrCardsInHand) _asbp_parent_card))
      (Variables|/Script/Project_CarDeer.ParentCard|SetPositionInHand _asbp_parent_card (Utilities|Array|Get(acopy) (Variables|Default|GetArrInHandPosition) _returnvalue_2)))))

(event EventPlayCard
  (bind _player_controller (Variables|Default|GetPlayer%20Controller))
  (bind _arrcardsinhand (Variables|Default|GetArrCardsInHand))
  (bind _card_in_hand (Variables|/Game/Blueprints/Player/BP_CarDeerPlayerController.BP_CarDeerPlayerController_C|GetCard%20In%20Hand _player_controller))
  ;[1 1 1] 出牌
  (Utilities|IsValid _card_in_hand
    (:Is%20Valid
      (bind _asbp_parent_card (Utilities|Casting|CastToBP_ParentCard _card_in_hand))
      (if (>= (Utilities|Array|FindItem _arrcardsinhand _asbp_parent_card) 0)
        (Class|ParentCard|Play _asbp_parent_card)
        (Utilities|Array|RemoveItem _arrcardsinhand _asbp_parent_card)
        (Variables|Default|SetNumOfCardsInHAnd (- (Variables|Default|GetNumOfCardsInHAnd) 1))
        (Class|BPIGameBasic|CardLaunchEffect(Message) _asbp_parent_card)))))

(event EventReleaseAbility
  (params (TargetUnit :type Map%20Unit%20Object%20Reference))
  (bind _glowingmapunits (Variables|Default|GetGlowingMapUnits))
  ;[1 1 1] 释放效果
  (|MatchMapUnit TargetUnit
    (:Success
      (Utilities|FlowControl|Sequence
        (:then_0
          (if (Variables|Default|GetCanMove)
            (Variables|Default|SetCanMove false)
            (for _array_element (Variables|Default|GetTarget%20Map%20Units)
              (Default|玩家棋子可移动格子指示器（需升起） _array_element false 2.0))
            (Class|BPICardEffect|PlayerMove(Message) (Variables|Default|GetPlayerChess) TargetUnit)
            (Utilities|Array|Clear (Variables|Default|GetTarget%20Map%20Units) :!label _label)
            (CallFunction|MakeMapUnitsDark _glowingmapunits)
            (Utilities|Array|Clear _glowingmapunits)
            (Variables|/Script/Project_CarDeer.Project_CarDeerPlayerController|SetCanPlayCard (Variables|Default|GetPlayer%20Controller) true)
            (Variables|Default|SetCanGlowMapUnit false)
            (if (== (Variables|Default|GetMana) 0)
              (Default|AnotherRound (Variables|Default|GetPlayer%20Controller)))))
        (:then_1
          (if (Variables|Default|GetCanAttack)
            (Variables|Default|SetCanAttack false)
            (for _array_element_2 (Variables|Default|GetTarget%20Map%20Units)
              (Default|玩家可攻击格子指示器（需升起） _array_element_2 false 2.0))
            (if (!= (Variables|Default|GetAttackMode) 4)
              (if (Variables|/Script/Project_CarDeer.MapUnit|GetbEnemySteppingOn TargetUnit)
                (Class|BPIChess|Damage(Message) (Variables|/Script/Project_CarDeer.MapUnit|GetActorSteppedOn TargetUnit) 1))
              (CallFunction|ChangeDigit TargetUnit)
              (CallFunction|PlayAttackFX (Actor|GetComponentbyClass TargetUnit "/Script/Engine.StaticMeshComponent"))
              (goto _label)
              (else
                (bind (_row _column) (Class|MapUnit|GetIndex TargetUnit))
                (bind _returnvalue (Class|MapArranger|GetTotalRowColUnitInstance (Variables|Default|GetMapArranger) _row _column))
                (for _array_element_3 _returnvalue
                  (if (Variables|/Script/Project_CarDeer.MapUnit|GetbEnemySteppingOn _array_element_3)
                    (Class|BPIChess|Damage(Message) (Variables|/Script/Project_CarDeer.MapUnit|GetActorSteppedOn _array_element_3) 3)
                    (CallFunction|PlayAttackFX (Actor|GetComponentbyClass _array_element_3 "/Script/Engine.StaticMeshComponent"))
                    (Variables|Default|SetAttackMode 0)))
                (goto _label)))))))))

(fn ConstructionScript)

(fn MakeCrossingMapUnitsGlow
  (params (TargetMap :type Map%20Unit%20Object%20Reference))
  (bind _returnvalue (Class|MapArranger|GetTotalRowColUnitInstance (Variables|Default|GetMapArranger) (Variables|/Script/Project_CarDeer.MapUnit|GetRowIndex TargetMap) (Variables|/Script/Project_CarDeer.MapUnit|GetColumnIndex TargetMap)))
  (for _array_element _returnvalue
    (bind _asbp_map_unit (Utilities|Casting|CastToBP_MapUnit _array_element))
    (Default|选中格子描边 _asbp_map_unit true)
    (Utilities|Array|Add (Variables|Default|GetGlowingMapUnits) _asbp_map_unit)))

(fn MakeColumnMapUnitsGlow
  (params (TargetMap :type Map%20Unit%20Object%20Reference))
  (bind _returnvalue (Class|MapArranger|GetColumnUnitInstance (Variables|Default|GetMapArranger) (Variables|/Script/Project_CarDeer.MapUnit|GetRowIndex TargetMap) (Variables|/Script/Project_CarDeer.MapUnit|GetColumnIndex TargetMap)))
  (for _array_element _returnvalue
    (bind _asbp_map_unit (Utilities|Casting|CastToBP_MapUnit _array_element))
    (Default|选中格子描边 _asbp_map_unit true)
    (Utilities|Array|Add (Variables|Default|GetGlowingMapUnits) _asbp_map_unit)))

(fn MakeRowMapUnitsGlow
  (params (TargetMap :type Map%20Unit%20Object%20Reference))
  (bind _returnvalue (Class|MapArranger|GetRowUnitInstance (Variables|Default|GetMapArranger) (Variables|/Script/Project_CarDeer.MapUnit|GetRowIndex TargetMap) (Variables|/Script/Project_CarDeer.MapUnit|GetColumnIndex TargetMap)))
  (for _array_element _returnvalue
    (bind _asbp_map_unit (Utilities|Casting|CastToBP_MapUnit _array_element))
    (Default|选中格子描边 _asbp_map_unit true)
    (Utilities|Array|Add (Variables|Default|GetGlowingMapUnits) _asbp_map_unit)))

(fn MakeMapUnitsDark
  (params (TargetMap :type Array%20of%20Map%20Unit%20Object%20References))
  (for _array_element TargetMap
    (bind _asbp_map_unit (Utilities|Casting|CastToBP_MapUnit _array_element))
    (Default|选中格子描边 _asbp_map_unit false)))

(fn MakeMapUnitsGlow
  (params (TargetGlowMap :type Map%20Unit%20Object%20Reference))
  (Utilities|FlowControl|Sequence
    (:then_0
      (if (== (Variables|Default|GetGlow%20Mode) 0)
        (bind _asbp_map_unit (Utilities|Casting|CastToBP_MapUnit TargetGlowMap))
        (Default|选中格子描边 _asbp_map_unit true)
        (Utilities|Array|Add (Variables|Default|GetGlowingMapUnits) _asbp_map_unit)))
    (:then_1
      (if (== (Variables|Default|GetGlow%20Mode) 1)
        (CallFunction|MakeRowMapUnitsGlow TargetGlowMap)))
    (:then_2
      (if (== (Variables|Default|GetGlow%20Mode) 2)
        (CallFunction|MakeColumnMapUnitsGlow TargetGlowMap)))
    (:then_3
      (if (== (Variables|Default|GetGlow%20Mode) 3)
        (bind (_row _column) (Class|MapUnit|GetIndex TargetGlowMap))
        (bind _outmapunits (CallFunction|GetManhattanDistanceMapUnits _row _column 1))
        (for _array_element _outmapunits
          (bind (_row_2 _column_2) (Class|MapUnit|GetIndex _array_element))
          (bind _returnvalue (Class|MapArranger|GetMapUnitInstance (Variables|Default|GetMapArranger) _row_2 _column_2))
          (bind _asbp_map_unit_2 (Utilities|Casting|CastToBP_MapUnit _returnvalue))
          (Default|选中格子描边 _asbp_map_unit_2 true)
          (Utilities|Array|Add (Variables|Default|GetGlowingMapUnits) _asbp_map_unit_2))))
    (:then_4
      (if (== (Variables|Default|GetGlow%20Mode) 4)
        (CallFunction|MakeCrossingMapUnitsGlow TargetGlowMap)))))

(fn ChangeDigit
  (params (UnitInstance :type Map%20Unit%20Object%20Reference))
  (if (== (Variables|Default|GetAttackMode) 0)
    (Class|MapArranger|AddUnitNum (Variables|Default|GetMapArranger) UnitInstance (Variables|Default|GetDigitChangeStep))
    (return)
    (elif (== (Variables|Default|GetAttackMode) 1)
      (bind (_row _column) (Class|MapUnit|GetIndex UnitInstance))
      (bind _returnvalue (Class|MapArranger|GetRowUnitInstance (Variables|Default|GetMapArranger) _row _column))
      (for _array_element _returnvalue
        (Class|MapArranger|AddUnitNum (Variables|Default|GetMapArranger) _array_element (Variables|Default|GetDigitChangeStep)))
      (return)
      (elif (== (Variables|Default|GetAttackMode) 2)
        (bind (_row_2 _column_2) (Class|MapUnit|GetIndex UnitInstance))
        (bind _returnvalue_2 (Class|MapArranger|GetColumnUnitInstance (Variables|Default|GetMapArranger) _row_2 _column_2))
        (for _array_element_2 _returnvalue_2
          (Class|MapArranger|AddUnitNum (Variables|Default|GetMapArranger) _array_element_2 (Variables|Default|GetDigitChangeStep)))
        (return)
        (elif (== (Variables|Default|GetAttackMode) 3)
          (bind (_row_3 _column_3) (Class|MapUnit|GetIndex UnitInstance))
          (bind _outmapunits (CallFunction|GetManhattanDistanceMapUnits _row_3 _column_3 1))
          (for _array_element_3 _outmapunits
            (bind (_row_4 _column_4) (Class|MapUnit|GetIndex _array_element_3))
            (bind _returnvalue_3 (Class|MapArranger|GetMapUnitInstance (Variables|Default|GetMapArranger) _row_4 _column_4))
            (Class|MapArranger|ClearUnitNum (Variables|Default|GetMapArranger) _returnvalue_3))
          (Class|MapArranger|ClearUnitNum (Variables|Default|GetMapArranger) UnitInstance)
          (return))))))

(fn PlayAttackFX
  (params (AttachToComponent :type Scene%20Component%20Object%20Reference))
  (Niagara|SpawnSystemAttached "/Game/VFX/NS_Attack.NS_Attack" AttachToComponent "None" "0, 0, 0" "0, 0, 0" "SnapToTarget" true true "AutoRelease"))

(fn DrawCard
  (params (CardClass :type Actor%20Class%20Reference))
  (return 0))