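; BP_ParentCard is a base card actor with an empty DrawCard function, apparently meant for child cards to override.
; On BeginPlay it caches the player chess piece, MapArranger and player pawn, and AddTargetMapUnits collects target map units from the arranger by row and column.
; BurnCard and DestroyCard share one path: after a short delay, a timeline drives a card material parameter and Niagara variable, then the actor is destroyed.
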(event Custom|Destroy%20Card
  (Utilities|FlowControl|Delay 0.5)
  (bind _tl_animatiion (Timeline|Timeline Play)
    (:Update
      (Rendering|Material|SetScalarParameterValueonMaterials (Variables|Default|GetCardMesh) "Animation" _tl_animatiion)
      (Niagara|SetNiagaraVariable(Float) (Variables|Default|GetNiagara) "User_Animation" _tl_animatiion)
      (Utilities|FlowControl|Delay 1.01)
      (Actor|DestroyActor))
    (:Finished
      (Actor|DestroyActor))))

(event EventBeginPlay
  (bind _outactors (Actor|GetAllActorsOfClass "/Game/Blueprints/Player/BP_PlayerChess.BP_PlayerChess_C"))
  (Variables|Default|SetPlayerChess (Utilities|Array|Get(acopy) _outactors))
  (bind _outactors_2 (Actor|GetAllActorsOfClass "/Script/Project_CarDeer.MapArranger"))
  (Variables|Default|SetMapArranger (Utilities|Array|Get(acopy) _outactors_2))
  (bind _asbp_player_pawn (Utilities|Casting|CastToBP_PlayerPawn (Game|Player|GetPlayerPawn 0)))
  (Variables|Default|SetPlayerPawn _asbp_player_pawn))

(event Collision|EventActorBeginOverlap
  (params (OtherActor :type Actor%20Object%20Reference)))

(event EventTick
  (params (DeltaSeconds :type Float%20%28single-precision%29)))

(event EventBurnCard
  (Utilities|FlowControl|Delay 0.5)
  (bind _tl_animatiion (Timeline|Timeline Play)
    (:Update
      (Rendering|Material|SetScalarParameterValueonMaterials (Variables|Default|GetCardMesh) "Animation" _tl_animatiion)
      (Niagara|SetNiagaraVariable(Float) (Variables|Default|GetNiagara) "User_Animation" _tl_animatiion)
      (Utilities|FlowControl|Delay 1.01)
      (Actor|DestroyActor))
    (:Finished
      (Actor|DestroyActor))))

(fn ConstructionScript)

(fn AddTargetMapUnits
  (params (row :type Integer) (col :type Integer))
  (bind _returnvalue (Class|MapArranger|GetMapUnitInstance (Variables|Default|GetMapArranger) row col))
  (bind _asbp_map_unit (Utilities|Casting|CastToBP_MapUnit _returnvalue))
  (Utilities|Array|Add (Variables|Default|GetTargetMapUnits) _asbp_map_unit))

(fn DrawCard
  (params (CardClass :type Actor%20Class%20Reference))
  (return 0))