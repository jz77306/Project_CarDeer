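; BP_EnemyCavalry is an enemy cavalry chess piece that hunts the player on a tile grid.
; Action picks a two-step orthogonal or one-step diagonal move toward the player, cycling through directions when tiles hold enemies.
; Direction macros resolve target tiles, and NewMacro transfers occupancy.
; Death frees the tile and queues the piece off-board via BP_EnemyArranger, while Tick triggers level loss when it shares the player's tile.
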(event EventBeginPlay
  (bind _outactors (Actor|GetAllActorsOfClass "/Game/Blueprints/Player/BP_PlayerChess.BP_PlayerChess_C"))
  (Variables|Default|SetTargetPlayerChess (Utilities|Array|Get(acopy) _outactors)))

(event EventChessRise
  (params (AnimationSecond :type Float%20%28double-precision%29))
  (bind _actorsequence (Variables|Default|GetActorSequence))
  (bind _sequenceplayer (Variables|/Script/ActorSequence.ActorSequenceComponent|GetSequencePlayer _actorsequence))
  ;[1 1 1] 棋子的上升下降
  (Components|Timeline|SetPlayRate _sequenceplayer AnimationSecond)
  (Sequencer|Player|Play _sequenceplayer :!class /Script/MovieScene.MovieSceneSequencePlayer))

(event EventChessHeightReset
  (params (AnimationSecond :type Float%20%28double-precision%29))
  ;[1 1 1] 棋子的上升下降
  (Class|MovieSceneSequencePlayer|PlayReverse (Variables|/Script/ActorSequence.ActorSequenceComponent|GetSequencePlayer (Variables|Default|GetActorSequence))))

(event EventShouldAction
  (bind _steppedonunit (Variables|Default|GetSteppedOnUnit))
  (CallFunction|Action)
  (Development|PrintString (Utilities|String|Append (Utilities|String|ToString(Integer) (Variables|/Script/Project_CarDeer.MapUnit|GetRowIndex _steppedonunit)) ", " (Utilities|String|ToString(Integer) (Variables|/Script/Project_CarDeer.MapUnit|GetColumnIndex _steppedonunit)))))

(event EventDamage
  (params (DamageAmount :type Integer))
  (bind _self self)
  (Class|EnemyPawn|TakeDamagefromPlayer DamageAmount)
  (if (Variables|Default|GetbIsDead)
    (bind _outactors (Actor|GetAllActorsOfClass "/Game/Blueprints/Enemy/BP_EnemyArranger.BP_EnemyArranger_C"))
    (Utilities|Array|RemoveItem (Variables|/Game/Blueprints/Enemy/BP_EnemyArranger.BP_EnemyArranger_C|GetPossessEnemyArray (Utilities|Array|Get(acopy) _outactors)) _self)
    (Variables|Default|SetDestination _self (Math|Vector|MakeVector (Math|Conversions|ToFloat(Integer) (+ (* (Variables|/Game/Blueprints/Enemy/BP_EnemyArranger.BP_EnemyArranger_C|GetNumOfEnemyQuit (Utilities|Array|Get(acopy) _outactors)) -100) (.x (Variables|/Game/Blueprints/Enemy/BP_EnemyArranger.BP_EnemyArranger_C|GetEnemyQuitQue (Utilities|Array|Get(acopy) _outactors))))) (.y (Variables|/Game/Blueprints/Enemy/BP_EnemyArranger.BP_EnemyArranger_C|GetEnemyQuitQue (Utilities|Array|Get(acopy) _outactors))) 0.0))
    (Variables|/Script/Project_CarDeer.MapUnit|SetbEnemySteppingOn (Variables|Default|GetSteppedOnUnit) false)
    (Variables|/Script/Project_CarDeer.MapUnit|SetActorSteppedOn (Variables|Default|GetSteppedOnUnit) 0)
    (Variables|Default|SetSteppedOnUnit 0)
    (Variables|/Game/Blueprints/Enemy/BP_EnemyArranger.BP_EnemyArranger_C|SetNumOfEnemyQuit (Utilities|Array|Get(acopy) _outactors) (+ (Variables|/Game/Blueprints/Enemy/BP_EnemyArranger.BP_EnemyArranger_C|GetNumOfEnemyQuit (Utilities|Array|Get(acopy) _outactors)) 1))
    (Class|BPIChess|EnemyQuit(Message) (Utilities|Array|Get(acopy) _outactors))))

(event EventTick
  (params (DeltaSeconds :type Float%20%28single-precision%29))
  (if (Variables|/Script/Project_CarDeer.MapUnit|GetbPlayerSteppingOn (Variables|Default|GetSteppedOnUnit))
    (Utilities|FlowControl|DoOnce false
      (:Completed
        (Utilities|FlowControl|Delay 2.0)
        (Class|BPIGameBasic|LevelLose(Message) (Game|GetPlayerController 0))))))

(fn ConstructionScript)

(fn Action
  (bind _targetplayerchess (Variables|Default|GetTargetPlayerChess))
  (bind _steppedonunit (Variables|Default|GetSteppedOnUnit))
  (bind _steppedonunit_2 (Variables|/Script/Project_CarDeer.PlayerChess|GetSteppedOnUnit _targetplayerchess))
  (bind _rowindex (Variables|/Script/Project_CarDeer.MapUnit|GetRowIndex _steppedonunit))
  (bind _columnindex (Variables|/Script/Project_CarDeer.MapUnit|GetColumnIndex _steppedonunit))
  (bind _rowindex_2 (Variables|/Script/Project_CarDeer.MapUnit|GetRowIndex _steppedonunit_2))
  (bind _columnindex_2 (Variables|/Script/Project_CarDeer.MapUnit|GetColumnIndex _steppedonunit_2))
  (bind _returnvalue (- _columnindex_2 _columnindex))
  (bind _returnvalue_2 (- _rowindex_2 _rowindex))
  (bind _returnvalue_3 (> _returnvalue_2 0))
  (bind _returnvalue_4 (> _returnvalue 0))
  (bind _returnvalue_5 (== _returnvalue 0))
  (bind _returnvalue_6 (== _returnvalue_2 0))
  (bind _returnvalue_7 (< _returnvalue_2 0))
  (bind _returnvalue_8 (< _returnvalue 0))
  (bind _returnvalue_9 (and _returnvalue_3 _returnvalue_5))
  (bind _returnvalue_10 (and _returnvalue_7 _returnvalue_5))
  (bind _returnvalue_11 (and _returnvalue_6 _returnvalue_4))
  (bind _returnvalue_12 (and _returnvalue_6 _returnvalue_8))
  (bind _outactors (Actor|GetAllActorsOfClass "/Game/Blueprints/BlockMap/BP_MapArranger.BP_MapArranger_C"))
  (if (and _returnvalue_3 _returnvalue_4)
    (bind (_destination _stepped_on_unit) (Utilities|DownRight (Utilities|Array|Get(acopy) _outactors) :!label _label))
    (if (Variables|/Script/Project_CarDeer.MapUnit|GetbEnemySteppingOn _stepped_on_unit)
      (bind (_stepped_on_unit_2 _returnvalue_13) (Utilities|Right (Utilities|Array|Get(acopy) _outactors) :!label _label_2))
      (if (Variables|/Script/Project_CarDeer.MapUnit|GetbEnemySteppingOn _stepped_on_unit_2)
        (bind (_stepped_on_unit_3 _destination_2) (Utilities|UpRight (Utilities|Array|Get(acopy) _outactors) :!label _label_3))
        (if (Variables|/Script/Project_CarDeer.MapUnit|GetbEnemySteppingOn _stepped_on_unit_3)
          (bind (_stepped_on_unit_4 _returnvalue_14) (Utilities|Up (Utilities|Array|Get(acopy) _outactors) :!label _label_4))
          (if (Variables|/Script/Project_CarDeer.MapUnit|GetbEnemySteppingOn _stepped_on_unit_4)
            (bind (_stepped_on_unit_5 _destination_3) (Utilities|UpLeft (Utilities|Array|Get(acopy) _outactors) :!label _label_5))
            (if (Variables|/Script/Project_CarDeer.MapUnit|GetbEnemySteppingOn _stepped_on_unit_5)
              (bind (_stepped_on_unit_6 _returnvalue_15) (Utilities|Le4ft (Utilities|Array|Get(acopy) _outactors) :!label _label_6))
              (if (Variables|/Script/Project_CarDeer.MapUnit|GetbEnemySteppingOn _stepped_on_unit_6)
                (bind (_stepped_on_unit_7 _destination_4) (Utilities|DownLeft (Utilities|Array|Get(acopy) _outactors) :!label _label_7))
                (if (Variables|/Script/Project_CarDeer.MapUnit|GetbEnemySteppingOn _stepped_on_unit_7)
                  (bind (_stepped_on_unit_8 _returnvalue_16) (Utilities|Down (Utilities|Array|Get(acopy) _outactors) :!label _label_8))
                  (if (Variables|/Script/Project_CarDeer.MapUnit|GetbEnemySteppingOn _stepped_on_unit_8)
                    (goto _label)
                    (else
                      (Utilities|NewMacro _stepped_on_unit_8)
                      (Variables|Default|SetDestination _returnvalue_16)))
                  (else
                    (Utilities|NewMacro _stepped_on_unit_7)
                    (Variables|Default|SetDestination _destination_4)))
                (else
                  (Utilities|NewMacro _stepped_on_unit_6)
                  (Variables|Default|SetDestination _returnvalue_15)))
              (else
                (Utilities|NewMacro _stepped_on_unit_5)
                (Variables|Default|SetDestination _destination_3)))
            (else
              (Utilities|NewMacro _stepped_on_unit_4)
              (Variables|Default|SetDestination _returnvalue_14)))
          (else
            (Utilities|NewMacro _stepped_on_unit_3)
            (Variables|Default|SetDestination _destination_2)))
        (else
          (Utilities|NewMacro _stepped_on_unit_2)
          (Variables|Default|SetDestination _returnvalue_13)))
      (else
        (Utilities|NewMacro _stepped_on_unit)
        (Variables|Default|SetDestination _destination)))
    (return true)
    (elif (and _returnvalue_3 _returnvalue_8)
      (goto _label_7)
      (elif (and _returnvalue_7 _returnvalue_4)
        (goto _label_3)
        (elif (and _returnvalue_7 _returnvalue_8)
          (goto _label_5)
          (elif _returnvalue_9
            (if (and _returnvalue_9 (< (+ (Variables|/Script/Project_CarDeer.MapUnit|GetRowIndex (Variables|Default|GetSteppedOnUnit)) 2) 5))
              (goto _label_8)
              (else
                (goto _label_4)))
            (elif _returnvalue_10
              (if (and _returnvalue_10 (> (+ (Variables|/Script/Project_CarDeer.MapUnit|GetRowIndex (Variables|Default|GetSteppedOnUnit)) -2) -1))
                (goto _label_4)
                (else
                  (goto _label_8)))
              (elif _returnvalue_11
                (if (and _returnvalue_11 (< (+ (Variables|/Script/Project_CarDeer.MapUnit|GetColumnIndex (Variables|Default|GetSteppedOnUnit)) 2) 5))
                  (goto _label_2)
                  (else
                    (goto _label_6)))
                (elif _returnvalue_12
                  (if (and _returnvalue_12 (> (+ (Variables|/Script/Project_CarDeer.MapUnit|GetColumnIndex (Variables|Default|GetSteppedOnUnit)) -2) -1))
                    (goto _label_6)
                    (else
                      (goto _label_2))))))))))))