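; Enemy soldier chess piece that chases the player across the grid, triggering level loss when sharing the player's tile.
; Action steps one tile toward the player, choosing axes randomly on diagonals and cycling directions past enemy-occupied tiles, updating occupancy and Destination.
; Damage animates a dynamic-material health billboard; death frees the tile, enables physics and joins BP_EnemyArranger's quit queue.
; An ActorSequence raises and lowers the piece.
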(event EventBeginPlay
  (bind _outactors (Actor|GetAllActorsOfClass "/Game/Blueprints/Player/BP_PlayerChess.BP_PlayerChess_C"))
  (Variables|Default|SetTargetPlayerChess (Utilities|Array|Get(acopy) _outactors)))

(event EventChessRise
  (params (AnimationSecond :type Float%20%28double-precision%29))
  (bind _actorsequence (Variables|Default|GetActorSequence))
  (bind _sequenceplayer (Variables|/Script/ActorSequence.ActorSequenceComponent|GetSequencePlayer _actorsequence))
  ;[1 1 1] 棋子的上升下降
  (Components|Timeline|SetPlayRate _sequenceplayer AnimationSecond)
  (Sequencer|Player|Play _sequenceplayer :!class /Script/MovieScene.MovieSceneSequencePlayer))

(event EventChessHeightReset
  (params (AnimationSecond :type Float%20%28double-precision%29))
  ;[1 1 1] 棋子的上升下降
  (Class|MovieSceneSequencePlayer|PlayReverse (Variables|/Script/ActorSequence.ActorSequenceComponent|GetSequencePlayer (Variables|Default|GetActorSequence))))

(event EventShouldAction
  (bind _steppedonunit (Variables|Default|GetSteppedOnUnit))
  (CallFunction|Action)
  (Development|PrintString (Utilities|String|Append (Utilities|String|ToString(Integer) (Variables|/Script/Project_CarDeer.MapUnit|GetRowIndex _steppedonunit)) ", " (Utilities|String|ToString(Integer) (Variables|/Script/Project_CarDeer.MapUnit|GetColumnIndex _steppedonunit)))))

(event EventDamage
  (params (DamageAmount :type Integer))
  (bind _self self)
  (Variables|Default|SetPreviousHP (Math|Conversions|ToFloat(Integer) (Variables|Default|GetBlood)))
  (Class|EnemyPawn|TakeDamagefromPlayer DamageAmount)
  (Utilities|FlowControl|Sequence
    (:then_0
      (bind _newtrack_0 (Timeline|Timeline PlayFromStart)
        (:Update
          (Rendering|Material|SetScalarParameterValue (Variables|Default|GetMDI_HP) "NormalizedHP" (/ (Math|Float|Lerp (Variables|Default|GetPreviousHP) (Math|Conversions|ToFloat(Integer) (Variables|Default|GetBlood)) _newtrack_0) (Variables|Default|GetTotalHP)) :!class /Script/Engine.MaterialInstanceDynamic))))
    (:then_1
      (if (Variables|Default|GetbIsDead)
        (bind _outactors (Actor|GetAllActorsOfClass "/Game/Blueprints/Enemy/BP_EnemyArranger.BP_EnemyArranger_C"))
        (Utilities|Array|RemoveItem (Variables|/Game/Blueprints/Enemy/BP_EnemyArranger.BP_EnemyArranger_C|GetPossessEnemyArray (Utilities|Array|Get(acopy) _outactors)) _self)
        (Variables|Default|SetDestination _self (Math|Vector|MakeVector (Math|Conversions|ToFloat(Integer) (+ (* (Variables|/Game/Blueprints/Enemy/BP_EnemyArranger.BP_EnemyArranger_C|GetNumOfEnemyQuit (Utilities|Array|Get(acopy) _outactors)) -100) (.x (Variables|/Game/Blueprints/Enemy/BP_EnemyArranger.BP_EnemyArranger_C|GetEnemyQuitQue (Utilities|Array|Get(acopy) _outactors))))) (.y (Variables|/Game/Blueprints/Enemy/BP_EnemyArranger.BP_EnemyArranger_C|GetEnemyQuitQue (Utilities|Array|Get(acopy) _outactors))) 0.0))
        (Utilities|FlowControl|Sequence
          (:then_0
            (Utilities|FlowControl|Delay 0.5)
            (Physics|SetSimulatePhysics (Variables|Default|Get立方体_材质_005) true))
          (:then_1
            (Variables|/Script/Project_CarDeer.MapUnit|SetbEnemySteppingOn (Variables|Default|GetSteppedOnUnit) false)
            (Variables|/Script/Project_CarDeer.MapUnit|SetActorSteppedOn (Variables|Default|GetSteppedOnUnit) 0)
            (Variables|Default|SetSteppedOnUnit 0)
            (Variables|/Game/Blueprints/Enemy/BP_EnemyArranger.BP_EnemyArranger_C|SetNumOfEnemyQuit (Utilities|Array|Get(acopy) _outactors) (+ (Variables|/Game/Blueprints/Enemy/BP_EnemyArranger.BP_EnemyArranger_C|GetNumOfEnemyQuit (Utilities|Array|Get(acopy) _outactors)) 1))
            (Class|BPIChess|EnemyQuit(Message) (Utilities|Array|Get(acopy) _outactors))))))))

(event EventTick
  (params (DeltaSeconds :type Float%20%28single-precision%29))
  (if (not (Variables|Default|GetbIsDead))
    (if (Variables|/Script/Project_CarDeer.MapUnit|GetbPlayerSteppingOn (Variables|Default|GetSteppedOnUnit))
      (Utilities|FlowControl|DoOnce false
        (:Completed
          (Utilities|FlowControl|Delay 2.0)
          (Class|BPIGameBasic|LevelLose(Message) (Game|GetPlayerController 0)))))))

(fn ConstructionScript
  (bind _blood (Variables|Default|GetBlood))
  (bind _returnvalue (Math|Conversions|ToFloat(Integer) _blood))
  (bind _returnvalue_2 (Rendering|Material|CreateDynamicMaterialInstance "/Game/Materials/M_HP.M_HP" "None" "None" :!class /Script/Engine.KismetMaterialLibrary))
  (bind _output_get (Variables|Default|SetMDI_HP _returnvalue_2))
  (Rendering|Material|SetMaterial (Variables|Default|GetMaterialBillboard) 0 _output_get)
  (Rendering|Material|SetScalarParameterValue (Variables|Default|GetMDI_HP) "TotalHP" _returnvalue :!class /Script/Engine.MaterialInstanceDynamic)
  (Variables|Default|SetTotalHP _returnvalue))

(fn Action
  (bind _outactors (Actor|GetAllActorsOfClass "/Game/Blueprints/BlockMap/BP_MapArranger.BP_MapArranger_C"))
  (if (and (> (- (Variables|/Script/Project_CarDeer.MapUnit|GetRowIndex (Variables|/Script/Project_CarDeer.PlayerChess|GetSteppedOnUnit (Variables|Default|GetTargetPlayerChess))) (Variables|/Script/Project_CarDeer.MapUnit|GetRowIndex (Variables|Default|GetSteppedOnUnit))) 0) (== (- (Variables|/Script/Project_CarDeer.MapUnit|GetColumnIndex (Variables|/Script/Project_CarDeer.PlayerChess|GetSteppedOnUnit (Variables|Default|GetTargetPlayerChess))) (Variables|/Script/Project_CarDeer.MapUnit|GetColumnIndex (Variables|Default|GetSteppedOnUnit))) 0))
    (bind (_next_unit _returnvalue) (Utilities|Down (Utilities|Array|Get(acopy) _outactors) :!label _label))
    (if (Variables|/Script/Project_CarDeer.MapUnit|GetbEnemySteppingOn _next_unit)
      (bind (_stepped_on_unit _returnvalue_2) (Utilities|Left (Utilities|Array|Get(acopy) _outactors) :!label _label_2))
      (Development|PrintString "Left")
      (if (Variables|/Script/Project_CarDeer.MapUnit|GetbEnemySteppingOn _stepped_on_unit)
        (bind (_stepped_on_unit_2 _returnvalue_3) (Utilities|Up (Utilities|Array|Get(acopy) _outactors) :!label _label_3))
        (if (Variables|/Script/Project_CarDeer.MapUnit|GetbEnemySteppingOn _stepped_on_unit_2)
          (bind (_stepped_on_unit_3 _returnvalue_4) (Utilities|Right (Utilities|Array|Get(acopy) _outactors) :!label _label_4))
          (if (Variables|/Script/Project_CarDeer.MapUnit|GetbEnemySteppingOn _stepped_on_unit_3)
            (goto _label)
            (else
              (Variables|/Script/Project_CarDeer.MapUnit|SetbEnemySteppingOn _stepped_on_unit_3 true)
              (Variables|/Script/Project_CarDeer.MapUnit|SetActorSteppedOn (Variables|Default|GetSteppedOnUnit) 0)
              (Variables|/Script/Project_CarDeer.MapUnit|SetbEnemySteppingOn (Variables|Default|GetSteppedOnUnit) false)
              (Variables|/Script/Project_CarDeer.MapUnit|SetActorSteppedOn _stepped_on_unit_3 self)
              (Variables|Default|SetSteppedOnUnit _stepped_on_unit_3)
              (Variables|Default|SetDestination _returnvalue_4)))
          (else
            (Variables|/Script/Project_CarDeer.MapUnit|SetbEnemySteppingOn _stepped_on_unit_2 true)
            (Variables|/Script/Project_CarDeer.MapUnit|SetActorSteppedOn (Variables|Default|GetSteppedOnUnit) 0)
            (Variables|/Script/Project_CarDeer.MapUnit|SetbEnemySteppingOn (Variables|Default|GetSteppedOnUnit) false)
            (Variables|/Script/Project_CarDeer.MapUnit|SetActorSteppedOn _stepped_on_unit_2 self)
            (Variables|Default|SetSteppedOnUnit _stepped_on_unit_2)
            (Variables|Default|SetDestination _returnvalue_3)))
        (else
          (Variables|/Script/Project_CarDeer.MapUnit|SetbEnemySteppingOn _stepped_on_unit true)
          (Variables|/Script/Project_CarDeer.MapUnit|SetActorSteppedOn (Variables|Default|GetSteppedOnUnit) 0)
          (Variables|/Script/Project_CarDeer.MapUnit|SetbEnemySteppingOn (Variables|Default|GetSteppedOnUnit) false)
          (Variables|/Script/Project_CarDeer.MapUnit|SetActorSteppedOn _stepped_on_unit self)
          (Variables|Default|SetSteppedOnUnit _stepped_on_unit)
          (Variables|Default|SetDestination _returnvalue_2)))
      (else
        (Variables|/Script/Project_CarDeer.MapUnit|SetbEnemySteppingOn _next_unit true)
        (Variables|/Script/Project_CarDeer.MapUnit|SetActorSteppedOn (Variables|Default|GetSteppedOnUnit) 0)
        (Variables|/Script/Project_CarDeer.MapUnit|SetbEnemySteppingOn (Variables|Default|GetSteppedOnUnit) false)
        (Variables|/Script/Project_CarDeer.MapUnit|SetActorSteppedOn _next_unit self)
        (Variables|Default|SetSteppedOnUnit _next_unit)
        (Variables|Default|SetDestination _returnvalue)))
    (return true)
    (elif (and (< (- (Variables|/Script/Project_CarDeer.MapUnit|GetRowIndex (Variables|/Script/Project_CarDeer.PlayerChess|GetSteppedOnUnit (Variables|Default|GetTargetPlayerChess))) (Variables|/Script/Project_CarDeer.MapUnit|GetRowIndex (Variables|Default|GetSteppedOnUnit))) 0) (== (- (Variables|/Script/Project_CarDeer.MapUnit|GetColumnIndex (Variables|/Script/Project_CarDeer.PlayerChess|GetSteppedOnUnit (Variables|Default|GetTargetPlayerChess))) (Variables|/Script/Project_CarDeer.MapUnit|GetColumnIndex (Variables|Default|GetSteppedOnUnit))) 0))
      (goto _label_3)
      (elif (and (== (- (Variables|/Script/Project_CarDeer.MapUnit|GetRowIndex (Variables|/Script/Project_CarDeer.PlayerChess|GetSteppedOnUnit (Variables|Default|GetTargetPlayerChess))) (Variables|/Script/Project_CarDeer.MapUnit|GetRowIndex (Variables|Default|GetSteppedOnUnit))) 0) (> (- (Variables|/Script/Project_CarDeer.MapUnit|GetColumnIndex (Variables|/Script/Project_CarDeer.PlayerChess|GetSteppedOnUnit (Variables|Default|GetTargetPlayerChess))) (Variables|/Script/Project_CarDeer.MapUnit|GetColumnIndex (Variables|Default|GetSteppedOnUnit))) 0))
        (goto _label_4)
        (elif (and (== (- (Variables|/Script/Project_CarDeer.MapUnit|GetRowIndex (Variables|/Script/Project_CarDeer.PlayerChess|GetSteppedOnUnit (Variables|Default|GetTargetPlayerChess))) (Variables|/Script/Project_CarDeer.MapUnit|GetRowIndex (Variables|Default|GetSteppedOnUnit))) 0) (< (- (Variables|/Script/Project_CarDeer.MapUnit|GetColumnIndex (Variables|/Script/Project_CarDeer.PlayerChess|GetSteppedOnUnit (Variables|Default|GetTargetPlayerChess))) (Variables|/Script/Project_CarDeer.MapUnit|GetColumnIndex (Variables|Default|GetSteppedOnUnit))) 0))
          (goto _label_2)
          (elif (and (> (- (Variables|/Script/Project_CarDeer.MapUnit|GetRowIndex (Variables|/Script/Project_CarDeer.PlayerChess|GetSteppedOnUnit (Variables|Default|GetTargetPlayerChess))) (Variables|/Script/Project_CarDeer.MapUnit|GetRowIndex (Variables|Default|GetSteppedOnUnit))) 0) (> (- (Variables|/Script/Project_CarDeer.MapUnit|GetColumnIndex (Variables|/Script/Project_CarDeer.PlayerChess|GetSteppedOnUnit (Variables|Default|GetTargetPlayerChess))) (Variables|/Script/Project_CarDeer.MapUnit|GetColumnIndex (Variables|Default|GetSteppedOnUnit))) 0))
            (if (> (Math|Random|RandomFloat) 0.5)
              (goto _label_4)
              (else
                (goto _label)))
            (elif (and (> (- (Variables|/Script/Project_CarDeer.MapUnit|GetRowIndex (Variables|/Script/Project_CarDeer.PlayerChess|GetSteppedOnUnit (Variables|Default|GetTargetPlayerChess))) (Variables|/Script/Project_CarDeer.MapUnit|GetRowIndex (Variables|Default|GetSteppedOnUnit))) 0) (< (- (Variables|/Script/Project_CarDeer.MapUnit|GetColumnIndex (Variables|/Script/Project_CarDeer.PlayerChess|GetSteppedOnUnit (Variables|Default|GetTargetPlayerChess))) (Variables|/Script/Project_CarDeer.MapUnit|GetColumnIndex (Variables|Default|GetSteppedOnUnit))) 0))
              (if (> (Math|Random|RandomFloat) 0.5)
                (goto _label_2)
                (else
                  (goto _label)))
              (elif (and (< (- (Variables|/Script/Project_CarDeer.MapUnit|GetRowIndex (Variables|/Script/Project_CarDeer.PlayerChess|GetSteppedOnUnit (Variables|Default|GetTargetPlayerChess))) (Variables|/Script/Project_CarDeer.MapUnit|GetRowIndex (Variables|Default|GetSteppedOnUnit))) 0) (> (- (Variables|/Script/Project_CarDeer.MapUnit|GetColumnIndex (Variables|/Script/Project_CarDeer.PlayerChess|GetSteppedOnUnit (Variables|Default|GetTargetPlayerChess))) (Variables|/Script/Project_CarDeer.MapUnit|GetColumnIndex (Variables|Default|GetSteppedOnUnit))) 0))
                (if (> (Math|Random|RandomFloat) 0.5)
                  (goto _label_4)
                  (else
                    (goto _label_3)))
                (elif (and (< (- (Variables|/Script/Project_CarDeer.MapUnit|GetRowIndex (Variables|/Script/Project_CarDeer.PlayerChess|GetSteppedOnUnit (Variables|Default|GetTargetPlayerChess))) (Variables|/Script/Project_CarDeer.MapUnit|GetRowIndex (Variables|Default|GetSteppedOnUnit))) 0) (< (- (Variables|/Script/Project_CarDeer.MapUnit|GetColumnIndex (Variables|/Script/Project_CarDeer.PlayerChess|GetSteppedOnUnit (Variables|Default|GetTargetPlayerChess))) (Variables|/Script/Project_CarDeer.MapUnit|GetColumnIndex (Variables|Default|GetSteppedOnUnit))) 0))
                  (if (> (Math|Random|RandomFloat) 0.5)
                    (goto _label_2)
                    (else
                      (goto _label_3))))))))))))