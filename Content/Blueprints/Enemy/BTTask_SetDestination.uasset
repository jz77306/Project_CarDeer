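; Behavior tree task for enemies that sets the Destination blackboard vector one fixed step from the owner's current location.
; It checks the bMoveUp, bMoveDown, bMoveLeft and bMoveRight blackboard flags in priority order, offsetting along world X or Y for the first one set.
; Each matching branch finishes the task as failed, while no set flag leaves the task without a FinishExecute call.
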(event EventReceiveExecute
  (params (OwnerActor :type Actor%20Object%20Reference))
  (bind _returnvalue (Transformation|GetActorLocation OwnerActor))
  (bind _returnvalue_2 (AI|GetBlackboard OwnerActor))
  (bind _returnvalue_3 (Utilities|Name|MakeLiteralName "Destination"))
  (if (ScalableFloat|GetValueasBool _returnvalue_2 (Utilities|Name|MakeLiteralName "bMoveUp"))
    (AI|Components|Blackboard|SetValueasVector _returnvalue_2 _returnvalue_3 (+ _returnvalue "200.000000,0.000000,0.000000"))
    (AI|BehaviorTree|FinishExecute false :!label _label)
    (elif (ScalableFloat|GetValueasBool _returnvalue_2 (Utilities|Name|MakeLiteralName "bMoveDown"))
      (AI|Components|Blackboard|SetValueasVector _returnvalue_2 _returnvalue_3 (+ _returnvalue "-200.000000,0.000000,0.000000"))
      (goto _label)
      (elif (ScalableFloat|GetValueasBool _returnvalue_2 (Utilities|Name|MakeLiteralName "bMoveLeft"))
        (AI|Components|Blackboard|SetValueasVector _returnvalue_2 _returnvalue_3 (+ _returnvalue "0.000000,-200.000000,0.000000"))
        (goto _label)
        (elif (ScalableFloat|GetValueasBool _returnvalue_2 (Utilities|Name|MakeLiteralName "bMoveRight"))
          (AI|Components|Blackboard|SetValueasVector _returnvalue_2 _returnvalue_3 (+ _returnvalue "0.000000,200.000000,0.000000"))
          (goto _label))))))