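; Behavior Tree task that sets an EnemySoldier's movement direction flags toward its existing TargetPlayerChess.
; It compares X and Y locations and sets one Blackboard bool per axis: up or down for X, left or right for Y.
; A coin flip only swaps write order, so both branches yield identical flags.
; It never clears flags, and it finishes successfully unless the cast fails, which skips FinishExecute.
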(event EventReceiveExecute
  (params (OwnerActor :type Actor%20Object%20Reference))
  (bind _returnvalue (AI|GetBlackboard OwnerActor))
  (bind _returnvalue_2 (Transformation|GetActorLocation OwnerActor))
  (bind _asenemy_soldier (Utilities|Casting|CastToEnemySoldier OwnerActor))
  (if (> (Math|Random|RandomFloat) 0.5)
    ;[1 1 1] 先Y后X
    (if (> (.x (Transformation|GetActorLocation (Variables|/Script/Project_CarDeer.EnemyPawn|GetTargetPlayerChess _asenemy_soldier))) (.x _returnvalue_2))
      (AI|Components|Blackboard|SetValueasBool _returnvalue (Utilities|Name|MakeLiteralName "bMoveUp") true)
      (else
        (AI|Components|Blackboard|SetValueasBool _returnvalue (Utilities|Name|MakeLiteralName "bMoveDown") true)))
    (if (> (.y (Transformation|GetActorLocation (Variables|/Script/Project_CarDeer.EnemyPawn|GetTargetPlayerChess _asenemy_soldier))) (.y _returnvalue_2))
      (AI|Components|Blackboard|SetValueasBool _returnvalue (Utilities|Name|MakeLiteralName "bMoveLeft") true)
      (else
        (AI|Components|Blackboard|SetValueasBool _returnvalue (Utilities|Name|MakeLiteralName "bMoveRight") true)))
    (else
      ;[1 1 1] 先X后Y
      (if (> (.y (Transformation|GetActorLocation (Variables|/Script/Project_CarDeer.EnemyPawn|GetTargetPlayerChess _asenemy_soldier))) (.y _returnvalue_2))
        (AI|Components|Blackboard|SetValueasBool _returnvalue (Utilities|Name|MakeLiteralName "bMoveLeft") true)
        (else
          (AI|Components|Blackboard|SetValueasBool _returnvalue (Utilities|Name|MakeLiteralName "bMoveRight") true)))
      (if (> (.x (Transformation|GetActorLocation (Variables|/Script/Project_CarDeer.EnemyPawn|GetTargetPlayerChess _asenemy_soldier))) (.x _returnvalue_2))
        (AI|Components|Blackboard|SetValueasBool _returnvalue (Utilities|Name|MakeLiteralName "bMoveUp") true)
        (else
          (AI|Components|Blackboard|SetValueasBool _returnvalue (Utilities|Name|MakeLiteralName "bMoveDown") true)))))
  (AI|BehaviorTree|FinishExecute true))