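; Enemy arranger that runs the enemy phase, giving each enemy in PossessEnemyArray its turn in sequence.
; ActivateEnemies resets the index, then Activate messages one enemy to act, waits briefly and re-calls itself until the array ends, then notifies the player controller.
; EnemyQuit signals level success after a delay once the quit count equals the initial enemy count.
; The EnemyPawn gathering loop is unwired, and DrawCard is empty.
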(event Custom|Activate
  (bind _possessenemyarray (Variables|Default|GetPossessEnemyArray))
  (bind _index (Variables|Default|GetIndex))
  (Class|BPIChess|ShouldAction(Message) (Utilities|Array|Get(acopy) _possessenemyarray _index))
  (Utilities|FlowControl|Delay 1.5)
  (bind _result (Math|Integer|IncrementInt _index)
    (:%20%20
      (if (<= _result (Utilities|Array|LastIndex _possessenemyarray))
        (CallFunction|Activate)
        (else
          (CallFunction|FinishEnemyPhase))))))

(event Custom|FinishEnemyPhase
  (Class|BPIGameBasic|EnemyPhaseFinish(Message) (Game|GetPlayerController 0)))

(event EventBeginPlay)

(event EventEnemyQuit
  (if (== (Variables|Default|GetNumOfEnemyQuit) (Variables|Default|GetInitEnemyNum))
    (Utilities|FlowControl|Delay 2.0)
    (Class|BPIGameBasic|LevelSuccess(Message) (Game|GetPlayerController 0))))

(event EventActivateEnemies
  (Variables|Default|SetIndex 0)
  (CallFunction|Activate))

(fn ConstructionScript)

(fn DeliverMessage
  (params (Index :type Integer))
  (Class|BPIChess|ShouldAction(Message) (Utilities|Array|Get(acopy) (Variables|Default|GetPossessEnemyArray) Index)))

(fn DrawCard
  (params (CardClass :type Actor%20Class%20Reference))
  (return 0))