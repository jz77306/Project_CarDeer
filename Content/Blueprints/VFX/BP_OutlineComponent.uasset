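; Actor component that gives a static mesh a toggleable outline using an overlay material.
; Initilize adds a collision-free duplicate of the target mesh to the owner, snaps it to the target and applies OverlayMaterial to every slot.
; AddOutlineMaterial unhides the duplicate and passes color and bound through custom primitive data, both at index 0, so bound overwrites red.
; RemoveOutlineMaterial hides the duplicate again.
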(event EventBeginPlay)

(event EventTick
  (params (DeltaSeconds :type Float%20%28single-precision%29)))

(fn AddOutlineMaterial
  (params (Color :type Linear%20Color%20Structure) (Bound%28Optional%29 :type Float%20%28single-precision%29))
  (bind (_r _g _b _a) (Math|Color|BreakColor Color))
  (bind _outlinemesh (Variables|Default|GetOutLineMesh))
  (Development|SetHiddeninGame (Variables|Default|GetOutLineMesh) false false)
  ;[1 1 1] ColorTint
  (Rendering|Material|SetCustomPrimitiveDataVector4 _outlinemesh 0 (Math|Vector4|MakeVector4 _r _g _b _a))
  ;[1 1 1] Bound
  (Rendering|Material|SetCustomPrimitiveDataFloat _outlinemesh 0 Bound%28Optional%29))

(fn RemoveOutlineMaterial
  (Development|SetHiddeninGame (Variables|Default|GetOutLineMesh) true false))

(fn Initilize
  (params (TargetMesh :type Static%20Mesh%20Component%20Object%20Reference))
  (bind _returnvalue (Game|AddComponentbyClass (Components|GetOwner) "/Script/Engine.StaticMeshComponent" true))
  (Variables|Default|SetOutLineMesh _returnvalue)
  (Transformation|AttachComponentToComponent (Variables|Default|GetOutLineMesh) TargetMesh "None" "SnapToTarget" "SnapToTarget" "SnapToTarget" true)
  (Collision|SetCollisionEnabled (Variables|Default|GetOutLineMesh) "NoCollision")
  (Components|StaticMesh|SetStaticMesh (Variables|Default|GetOutLineMesh) (Variables|/Script/Engine.StaticMeshComponent|GetStaticMesh TargetMesh))
  (for _index (range 0 (Rendering|Material|GetNumMaterials (Variables|Default|GetOutLineMesh)))
    (Rendering|Material|SetMaterial (Variables|Default|GetOutLineMesh) _index (Variables|Default|GetOverlayMaterial))))