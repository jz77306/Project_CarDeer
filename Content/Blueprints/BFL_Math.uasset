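; Blueprint function library for grid math that finds map units at a given Manhattan distance from a row and column.
; GetManhattanDistanceMapUnits scans every BP_MapUnit actor in the level and collects those whose grid index passes the CalculateDistance check.
; CalculateDistance compares the summed absolute row and column differences to Step for equality, describing a diamond ring rather than a filled area.
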(fn GetManhattanDistanceMapUnits
  (params (Row :type Integer) (Column :type Integer) (Step :type Integer))
  (Utilities|Array|Clear (LocalVariables|GetTempMapUnits))
  (bind _outactors (Actor|GetAllActorsOfClass 0 "/Game/Blueprints/BlockMap/BP_MapUnit.BP_MapUnit_C"))
  (for _array_element _outactors
    (bind (_row _column) (Class|MapUnit|GetIndex _array_element))
    (if (|CalculateDistance _row _column Row Column)
      (Utilities|Array|Add (LocalVariables|GetTempMapUnits) _array_element)))
  (return (LocalVariables|GetTempMapUnits)))