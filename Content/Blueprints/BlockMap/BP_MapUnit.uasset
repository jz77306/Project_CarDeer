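; BP_MapUnit is a block-map grid cell that shows its number as text and displays board-game indicators for movement, attack and selection.
; Overlay components tint the mesh green for player moves and red for attack or enemy range, and outline selection in yellow.
; Move and attack indicators also play or reverse a floating sequence; move additionally signals the standing chess piece to rise or reset.
; Cursor hover test-triggers the enemy-range tint, while the number-change indicator is an empty stub.
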(event OnBeginCursorOver(StaticMesh)
  (params (TouchedComponent :type Primitive%20Component%20Object%20Reference))
  ;[1 0 0] TestOnly
  (FX|敌人可移动范围指示器（不用升起） true))

(event OnEndCursorOver(StaticMesh)
  (params (TouchedComponent :type Primitive%20Component%20Object%20Reference))
  ;[1 0 0] TestOnly
  (FX|敌人可移动范围指示器（不用升起） false))

(event EventBeginPlay)

(event Collision|EventActorBeginOverlap
  (params (OtherActor :type Actor%20Object%20Reference)))

(event EventTick
  (params (DeltaSeconds :type Float%20%28single-precision%29)))

(event EventUpdateUnitNumShow
  ;[1 1 1] 更新格子数字显示效果
  (Rendering|Components|TextRender|SetText (Variables|Default|GetTextRender) (Utilities|Text|ToText(Integer) (Class|MapUnit|GetUnitNum))))

(fn ConstructionScript)

(fn 玩家棋子可移动格子指示器（需升起）
  (params (Enable :type Boolean) (AnimationSecond :type Float%20%28double-precision%29))
  (bind _bp_overlaycolorcomponent (Variables|Default|GetBP_OverlayColorComponent))
  (bind _staticmesh (Variables|Default|GetStaticMesh))
  (CallFunction|FloatActor Enable AnimationSecond)
  (|对格子上的棋子进行升降)
  (if Enable
    (Default|AddOverlayMaterial _bp_overlaycolorcomponent "(R=0.008000,G=1.000000,B=0.000000,A=1.000000)" _staticmesh 1.0)
    (else
      (Default|RemoveOverlayMaterial _bp_overlaycolorcomponent _staticmesh))))

(fn 玩家可攻击格子指示器（需升起）
  (params (Enable :type Boolean) (AnimationSecond :type Float%20%28single-precision%29))
  (bind _bp_overlaycolorcomponent (Variables|Default|GetBP_OverlayColorComponent))
  (bind _staticmesh (Variables|Default|GetStaticMesh))
  (CallFunction|FloatActor Enable AnimationSecond)
  (if Enable
    (Default|AddOverlayMaterial _bp_overlaycolorcomponent "(R=1.000000,G=0.000000,B=0.000000,A=1.000000)" _staticmesh 1.0)
    (else
      (Default|RemoveOverlayMaterial _bp_overlaycolorcomponent _staticmesh))))

(fn 敌人可移动范围指示器（不用升起）
  (params (Enable :type Boolean))
  (bind _bp_overlaycolorcomponent (Variables|Default|GetBP_OverlayColorComponent))
  (bind _staticmesh (Variables|Default|GetStaticMesh))
  (if Enable
    (Default|AddOverlayMaterial _bp_overlaycolorcomponent "(R=1.000000,G=0.000000,B=0.000000,A=1.000000)" _staticmesh 1.0)
    (else
      (Default|RemoveOverlayMaterial _bp_overlaycolorcomponent _staticmesh))))

(fn 选中格子描边
  (params (Enbale :type Boolean))
  (bind _bp_outlinecomponent (Variables|Default|GetBP_OutLineComponent))
  (bind _staticmesh (Variables|Default|GetStaticMesh))
  (if Enbale
    (Default|AddOverlayMaterial _bp_outlinecomponent "(R=1.000000,G=1.000000,B=0.000000,A=1.000000)" _staticmesh 1.0)
    (else
      (Default|RemoveOverlayMaterial _bp_outlinecomponent _staticmesh))))

(fn 格子数字加减指示器（不用升起）)

(fn FloatActor
  (params (Enable :type Boolean) (Rate :type Float%20%28double-precision%29))
  (bind _floatingsequence (Variables|Default|GetFloatingSequence))
  (bind _sequenceplayer (Variables|/Script/ActorSequence.ActorSequenceComponent|GetSequencePlayer _floatingsequence))
  (Utilities|FlowControl|Sequence
    (:then_0
      (Development|PrintText (Utilities|Text|FormatText "{Name} Floating 
Reverse {bool}" (Utilities|GetDisplayName self) Enable)))
    (:then_1
      (LocalVariables|SetAnimationSecond (/ 1.0 (Math|Float|Max(Float) Rate 0.001)))
      (if Enable
        (Components|Timeline|SetPlayRate _sequenceplayer (LocalVariables|GetAnimationSecond))
        (Sequencer|Player|Play _sequenceplayer :!class /Script/MovieScene.MovieSceneSequencePlayer)
        (else
          (Class|MovieSceneSequencePlayer|PlayReverse _sequenceplayer)))
      (return (LocalVariables|GetAnimationSecond)))))