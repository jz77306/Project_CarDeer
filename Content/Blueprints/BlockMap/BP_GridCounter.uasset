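; BP_GridCounter is a block map actor that displays a number on a material billboard.
; Its construction script creates a dynamic instance of the M_Num material and applies it to the billboard.
; UpdateCountersNumShow pushes SumNum into the material's Index parameter and randomizes Strength on each call to vary the display effect.
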(event EventBeginPlay)

(event Collision|EventActorBeginOverlap
  (params (OtherActor :type Actor%20Object%20Reference)))

(event EventTick
  (params (DeltaSeconds :type Float%20%28single-precision%29)))

(event EventUpdateCountersNumShow
  (bind _mdi (Variables|Default|GetMDI))
  ;[1 1 1] 更新数字显示效果
  (Rendering|Material|SetScalarParameterValue _mdi "Index" (Math|Conversions|ToFloat(Integer) (Variables|Default|GetSumNum)) :!class /Script/Engine.MaterialInstanceDynamic)
  (Rendering|Material|SetScalarParameterValue _mdi "Strength" (Math|Random|RandomFloatinRange 0.2 0.6) :!class /Script/Engine.MaterialInstanceDynamic))

(fn ConstructionScript
  (bind _returnvalue (Rendering|Material|CreateDynamicMaterialInstance "/Game/VFX/M_Num.M_Num" "None" "None" :!class /Script/Engine.KismetMaterialLibrary))
  (bind _output_get (Variables|Default|SetMDI _returnvalue))
  (Rendering|Material|SetMaterial (Variables|Default|GetMaterialBillboard) 0 _output_get))