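; BP_MapCenter highlights the map tiles targeted by the mouse cursor, either a line sharing its row or column index or a single tile.
; Tick runs SwitchPattern, which picks matching BP_MapUnits by Pattern, and traces under the cursor to update the target index.
; Open/CloseChannel flip-flops a gate for cursor targeting, resetting the index on close.
; Highlighting works through the material scalar Lightness, cleared before each reselection.
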(event Custom|Open/CloseChannel
  ;[1 1 1] 射线检测鼠标指向的地块，并使目标地块高亮
  (Utilities|FlowControl|FlipFlop
    (:A
      (Utilities|FlowControl|Gate true :!label _label ; enters at Open
        (:Exit
          _)))
    (:B
      (Variables|Default|SetTargetMapUnitIndex "(X=-1.000000,Y=-1.000000)")
      (goto _label Close)))
  (bind _asbp_map_unit (Utilities|Casting|CastToBP_MapUnit (.HitActor (Collision|BreakHitResult (.HitResult (Game|Player|GetHitResultUnderCursorbyChannel (Game|GetPlayerController 0) "TraceTypeQuery1" true))))))
  (Variables|Default|SetTargetMapUnitIndex (Math|Vector2D|MakeVector2D (Math|Conversions|ToFloat(Integer) (.Column%20Index (|GetMapUnitIndex _asbp_map_unit))) (Math|Conversions|ToFloat(Integer) (.Row%20Index (|GetMapUnitIndex _asbp_map_unit))))))

(event Custom|GetAllMapUnitsWithRow
  ;[1 1 1] 获取一个、一行或者一列的地块
  (Utilities|MakeTargetMapUnitDark)
  (Utilities|Array|Clear (Variables|Default|GetTargetMapUnits))
  (for _array_element (Variables|Default|GetAllMapUnits)
    (if (== (.x (Variables|Default|GetTargetMapUnitIndex)) (Variables|/Script/Project_CarDeer.MapUnit|GetColumnIndex _array_element))
      (Utilities|Array|Add (Variables|Default|GetTargetMapUnits) _array_element)))
  (if (not (Utilities|Array|IsEmpty (Variables|Default|GetTargetMapUnits)))
    (CallFunction|ShowTargetMapUnit)))

(event Custom|GetAllMapUnitsWithColumn
  ;[1 1 1] 获取一个、一行或者一列的地块
  (Utilities|MakeTargetMapUnitDark)
  (Utilities|Array|Clear (Variables|Default|GetTargetMapUnits))
  (for _array_element (Variables|Default|GetAllMapUnits)
    (if (== (Variables|/Script/Project_CarDeer.MapUnit|GetRowIndex _array_element) (.y (Variables|Default|GetTargetMapUnitIndex)))
      (Utilities|Array|Add (Variables|Default|GetTargetMapUnits) _array_element)))
  (if (not (Utilities|Array|IsEmpty (Variables|Default|GetTargetMapUnits)))
    (CallFunction|ShowTargetMapUnit)))

(event Custom|GetTargetMapUnitWithIndex
  (bind _targetmapunitindex (Variables|Default|GetTargetMapUnitIndex))
  ;[1 1 1] 获取一个、一行或者一列的地块
  (Utilities|MakeTargetMapUnitDark)
  (Utilities|Array|Clear (Variables|Default|GetTargetMapUnits))
  (for _array_element (Variables|Default|GetAllMapUnits)
    (if (== (Variables|/Script/Project_CarDeer.MapUnit|GetColumnIndex _array_element) (.x _targetmapunitindex))
      (if (== (Variables|/Script/Project_CarDeer.MapUnit|GetRowIndex _array_element) (.y _targetmapunitindex))
        (Utilities|Array|Add (Variables|Default|GetTargetMapUnits) _array_element))))
  (if (not (Utilities|Array|IsEmpty (Variables|Default|GetTargetMapUnits)))
    (CallFunction|ShowTargetMapUnit)))

(event Custom|ShowTargetMapUnit
  (Utilities|MakeTargetMapUnitGlow))

(event EventBeginPlay
  (bind _outactors (Actor|GetAllActorsOfClass "/Game/Blueprints/BlockMap/BP_MapArranger.BP_MapArranger_C"))
  (Variables|Default|SetMapArranger (Utilities|Array|Get(acopy) _outactors))
  (bind _outactors_2 (Actor|GetAllActorsOfClass "/Game/Blueprints/BlockMap/BP_MapUnit.BP_MapUnit_C"))
  (Variables|Default|SetAllMapUnits _outactors_2))

(event EventTick
  (params (DeltaSeconds :type Float%20%28single-precision%29))
  ;[1 1 1] 射线检测鼠标指向的地块，并使目标地块高亮
  (Utilities|SwitchPattern)
  (bind _asbp_map_unit (Utilities|Casting|CastToBP_MapUnit (.HitActor (Collision|BreakHitResult (.HitResult (Game|Player|GetHitResultUnderCursorbyChannel (Game|GetPlayerController 0) "TraceTypeQuery1" true))))))
  (Variables|Default|SetTargetMapUnitIndex (Math|Vector2D|MakeVector2D (Math|Conversions|ToFloat(Integer) (.Column%20Index (|GetMapUnitIndex _asbp_map_unit))) (Math|Conversions|ToFloat(Integer) (.Row%20Index (|GetMapUnitIndex _asbp_map_unit))))))

(fn ConstructionScript)