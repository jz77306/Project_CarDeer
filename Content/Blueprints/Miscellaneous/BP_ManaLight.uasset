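; BP_ManaLight displays the player's mana as four lights and starts the BGM on BeginPlay.
; ManaChange compares PlayerPawn's Mana with the displayed NowMana and routes the difference to RestoredMana or UsingMana.
; These events recursively step through timeline-driven macros, Mana++ and Mana--, fading each light's material Lightness up or down.
; Each step updates NowMana when its timeline finishes, clamping it between zero and four.
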(event Custom|Using%20Mana
  (params (Manachange :type Integer))
  (if (> (Variables|Default|GetNowMana) 0)
    (|Mana--
      (:%20%20
        (bind _result (Math|Integer|DecrementInt Manachange)
          (:%20%20
            (if (!= _result 0)
              (CallFunction|UsingMana _result))))))))

(event Custom|Restored%20Mana
  (params (Manachange :type Integer))
  (if (< (Variables|Default|GetNowMana) 4)
    (|Mana++
      (:%20%20
        (bind _result (Math|Integer|DecrementInt Manachange)
          (:%20%20
            (if (!= _result 0)
              (CallFunction|RestoredMana _result))))))))

(event EventBeginPlay
  (Audio|Components|Audio|Play (Variables|Default|GetBGM) 0.0)
  (bind _asplayer_pawn (Utilities|Casting|CastToPlayerPawn (Game|Player|GetPlayerPawn 0)))
  (Variables|Default|SetPlayer%20Pawn _asplayer_pawn)
  (Variables|Default|SetLights (Utilities|Array|MakeArray (Variables|Default|GetLIght_01) (Variables|Default|GetLIght_02) (Variables|Default|GetLIght_03) (Variables|Default|GetLIght_04))))

(event EventManaChange
  (bind _nowmana (Variables|Default|GetNowMana))
  (bind _player_pawn (Variables|Default|GetPlayer%20Pawn))
  (bind _mana (Variables|/Script/Project_CarDeer.PlayerPawn|GetMana _player_pawn))
  (bind _returnvalue (- _mana _nowmana))
  (if (> _returnvalue 0)
    (CallFunction|RestoredMana _returnvalue)
    (else
      (CallFunction|UsingMana (Math|Integer|Absolute(Integer) _returnvalue)))))

(fn ConstructionScript)

(fn DrawCard
  (params (CardClass :type Actor%20Class%20Reference))
  (return 0))