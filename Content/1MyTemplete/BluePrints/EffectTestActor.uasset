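; An effect test actor that previews a material or Niagara system in the level with a text label naming it.
; The construction script applies the exposed mesh, material and scale to a plane, offsets it vertically by scale, and shows it only when the material is valid.
; It also assigns the Niagara system and labels the actor with the material name, falling back to the system name.
; The event graph is empty.
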(event EventBeginPlay)

(event Collision|EventActorBeginOverlap
  (params (OtherActor :type Actor%20Object%20Reference)))

(event EventTick
  (params (DeltaSeconds :type Float%20%28single-precision%29)))

(fn ConstructionScript
  (bind _plane (Variables|Default|GetPlane))
  (bind _scale (Variables|Default|GetScale))
  (bind _material (Variables|Default|GetMaterial))
  (bind _returnvalue (Utilities|IsValid _material))
  (Components|StaticMesh|SetStaticMesh (Variables|Default|GetPlane) (Variables|Default|GetMesh))
  (Rendering|Components|TextRender|SetWorldSize (Variables|Default|GetTextRender) (Variables|Default|GetSize))
  (Rendering|Material|SetMaterial (Variables|Default|GetPlane) 0 _material)
  (Transformation|SetWorldScale3D _plane _scale)
  (Transformation|SetRelativeLocation _plane (Math|Vector|MakeVector 0.0 0.0 (* (.Y (Math|Vector|BreakVector _scale)) -5e+01)) false false)
  (Rendering|SetVisibility (Variables|Default|GetPlane) _returnvalue false)
  (Class|NiagaraComponent|SetAsset (Variables|Default|GetNiagara) (Variables|Default|GetSystem) true)
  (Rendering|Components|TextRender|SetText (Variables|Default|GetTextRender) (Utilities|Text|ToText(String) (Utilities|String|SelectString (Utilities|GetObjectName _material) (Utilities|GetObjectName (Effects|Components|ParticleSystem|GetFXSystemAsset (Variables|Default|GetNiagara))) _returnvalue))))