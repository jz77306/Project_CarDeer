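; Base gameplay cue actor that fires optional effects on BeginPlay: post-process, fading decal, sound, Niagara and world camera shake, each toggled by a flag.
; Construction creates dynamic decal and post-process materials; the latter receives spawn time, lifetime, radius and actor position for time- and location-driven effects.
; Decals and Niagara spawn attached or at location, and TransferNiagaraParam pushes generic float and vector parameters into the stored, non-attached Niagara system.
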(event EventBeginPlay
  (CallFunction|SpawnPostFX)
  (CallFunction|SpawnDecal)
  (CallFunction|SpawnSound)
  (CallFunction|SpawnNiagara)
  (CallFunction|SpawnCameraShake))

(event Collision|EventActorBeginOverlap
  (params (OtherActor :type Actor%20Object%20Reference)))

(event EventTick
  (params (DeltaSeconds :type Float%20%28single-precision%29)))

(fn ConstructionScript
  (CallFunction|InitializePost)
  (CallFunction|InitialzeDecal))

(fn SpawnPostFX
  (bind _postmatmid (Variables|Post|GetPostMatMID))
  (bind _postmatmid_2 (Variables|Post|GetPostMatMID))
  (if (Variables|Post|GetApplyPostFX?)
    (Rendering|Material|SetScalarParameterValue _postmatmid_2 "SpawnTime" (Utilities|Time|GetGameTimeinSeconds) :!class /Script/Engine.MaterialInstanceDynamic)
    (Rendering|Material|SetScalarParameterValue _postmatmid_2 "LifeTime" (Variables|Post|GetPostLifeSpan) :!class /Script/Engine.MaterialInstanceDynamic)
    (Rendering|Material|SetScalarParameterValue _postmatmid "Radius" (Variables|Post|GetPostRadius) :!class /Script/Engine.MaterialInstanceDynamic)
    (Rendering|Material|SetVectorParameterValue _postmatmid "ObjectPosition" (Math|Conversions|ToLinearColor(Vector) (Transformation|GetActorLocation)) :!class /Script/Engine.MaterialInstanceDynamic)))

(fn SpawnDecal
  (params (AttachToComponent :type Scene%20Component%20Object%20Reference))
  (bind _returnvalue (Math|Random|RandomFloatinRange 0.0 3.6e+02))
  (bind _randomrotate_ (Variables|Decal|GetRandomRotate?))
  (bind _returnvalue_2 (Math|Rotator|MakeRotator _returnvalue -9e+01 0.0))
  (bind _returnvalue_3 (select _randomrotate_ _returnvalue_2 "-90.000000,0.000000,0.000000"))
  (if (Variables|Decal|GetApplyDecal?)
    (if (Variables|Decal|GetDecalAttached?)
      (bind _returnvalue_4 (Class|GameplayStatics|SpawnDecalAttached (Variables|Decal|GetDecalMatMID) (Variables|Decal|GetDecal%20Size) AttachToComponent "None" (Transformation|GetActorLocation) _returnvalue_3 "SnapToTarget" 0.0))
      (Rendering|Components|Decal|SetFadeOut _returnvalue_4 0.0 (Variables|Decal|GetDecal%20Life%20Span) true)
      (else
        (bind _returnvalue_5 (Rendering|Decal|SpawnDecalatLocation (Variables|Decal|GetDecalMatMID) (Variables|Decal|GetDecal%20Size) (Transformation|GetActorLocation) _returnvalue_3 (Variables|Decal|GetDecal%20Life%20Span)))
        (Rendering|Components|Decal|SetFadeOut _returnvalue_5 0.0 (Variables|Decal|GetDecal%20Life%20Span) true)))))

(fn SpawnSound
  (if (Variables|Sound|GetApplySound?)
    (Audio|PlaySoundatLocation (Variables|Sound|GetSound) (Transformation|GetActorLocation) "0, 0, 0" 1.0 1.0 0.0 0 0 0 0)))

(fn SpawnNiagara
  (params (AttachToComponent :type Scene%20Component%20Object%20Reference))
  (if (Variables|Niagara|GetApplyNiagara?)
    (if (Variables|Niagara|GetNiagaraAttached?)
      (Niagara|SpawnSystemAttached (Variables|Niagara|GetNiagaraSystem) AttachToComponent "None" "0, 0, 0" "0, 0, 0" "SnapToTarget" true)
      (else
        (bind _returnvalue (Niagara|SpawnSystematLocation (Variables|Niagara|GetNiagaraSystem) (Transformation|GetActorLocation)))
        (Variables|Default|SetSpawnedNiagara _returnvalue)))))

(fn SpawnCameraShake
  (if (Variables|CameraShake|GetApplyCameraShake?)
    (Camera|PlayWorldCameraShake (Variables|CameraShake|GetCameraShake) (Transformation|GetActorLocation) (Variables|CameraShake|GetInner%20Radius) (Variables|CameraShake|GetOuter%20Radius) (Variables|CameraShake|GetFalloff))))

(fn InitializePost
  (if (Variables|Post|GetApplyPostFX?)
    (bind _returnvalue (Rendering|Material|CreateDynamicMaterialInstance (Variables|Post|GetPostMat) "None" "None" :!class /Script/Engine.KismetMaterialLibrary))
    (Variables|Post|SetPostMatMID _returnvalue)
    (bind _returnvalue_2 (AddComponent|AddPostProcessComponent false))
    (bind _output_get (Variables|Components|SetPostVolume _returnvalue_2))
    (Variables|/Script/Engine.PostProcessComponent|SetSettings _output_get (|SetPostMat))
    (elif (not (== (Variables|Components|GetPostVolume) 0))
      (Components|DestroyComponent (Variables|Components|GetPostVolume)))))

(fn OnActive
  (params (MyTarget :type Actor%20Object%20Reference) (Parameters :type Gameplay%20Cue%20Parameters%20Structure%20%28by%20ref%29))
  (return false))

(fn InitialzeDecal
  (bind _returnvalue (Rendering|Material|CreateDynamicMaterialInstance (Variables|Decal|GetDecal%20Material) "None" "None" :!class /Script/Engine.KismetMaterialLibrary))
  (Variables|Decal|SetDecalMatMID _returnvalue))

(fn TransferNiagaraParam
  (params (InParam :type Struct%20Niagara%20Param%20Structure))
  (bind (_float0 _float1 _float2 _vector0 _vector1) (Utilities|Struct|BreakStruct_NiagaraParam InParam))
  (bind _spawnedniagara (Variables|Default|GetSpawnedNiagara))
  (Utilities|IsValid (Variables|Default|GetSpawnedNiagara)
    (:Is%20Valid
      (Utilities|FlowControl|Sequence
        (:then_0
          (Niagara|SetNiagaraVariable(Float) _spawnedniagara "Float0" _float0)
          (Niagara|SetNiagaraVariable(Float) _spawnedniagara "Float1" _float1)
          (Niagara|SetNiagaraVariable(Float) _spawnedniagara "Float2" _float2))
        (:then_1
          (Niagara|SetNiagaraVariable(Vector3) _spawnedniagara "Vector0" _vector0)
          (Niagara|SetNiagaraVariable(Vector3) _spawnedniagara "Vector1" _vector1))))))