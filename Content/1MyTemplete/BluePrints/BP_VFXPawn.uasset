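; Pawn for previewing Niagara VFX, with debug hotkeys for time, view modes and effect replay.
; Number keys toggle a ViewMode scalar in the MPC_PPVTest parameter collection, with the current mode printed every tick.
; Tab toggles global slow motion while raising the pawn's own time dilation to compensate.
; F restarts all Niagara actors, and Shift+Tab toggles cursor and UI input.
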(event EventTick
  (params (DeltaSeconds :type Float%20%28single-precision%29))
  (Development|PrintText (Utilities|Text|ToText(String) (Utilities|String|Append "CurrentViewMode:" (Utilities|String|EnumtoString (Variables|Default|GetViewMode)))) true true "(R=0.000000,G=0.660000,B=1.000000,A=1.000000)" DeltaSeconds))

(event Collision|EventActorBeginOverlap
  (params (OtherActor :type Actor%20Object%20Reference)))

(event Input|KeyboardEvents|Tab
  (params (Key :type Key%20Structure :default "None"))
  (:Pressed
    (Utilities|FlowControl|FlipFlop
      (:A
        (Utilities|Time|SetGlobalTimeDilation 0.1)
        (Variables|/Script/Engine.MovementComponent|SetVelocity (Variables|Default|GetMovementComponent) "0, 0, 0")
        (Variables|Default|SetCustomTimeDilation 1e+01))
      (:B
        (Utilities|Time|SetGlobalTimeDilation 1.0)
        (Variables|Default|SetCustomTimeDilation 1.0)))))

(event Input|KeyboardEvents|F
  (params (Key :type Key%20Structure :default "None"))
  (:Pressed
    (bind _outactors (Actor|GetAllActorsOfClass "/Script/Niagara.NiagaraActor"))
    (for _array_element _outactors
      (Components|Activation|Deactivate (Variables|/Script/Niagara.NiagaraActor|GetNiagaraComponent _array_element))
      (Components|Activation|SetActive (Variables|/Script/Niagara.NiagaraActor|GetNiagaraComponent _array_element) true true))))

(event Input|KeyboardEvents|ShiftTab
  (params (Key :type Key%20Structure :default "None"))
  (bind _returnvalue (Game|GetPlayerController 0))
  (bind _returnvalue_2 (Game|GetPlayerController 0))
  (:Pressed
    (Utilities|FlowControl|FlipFlop
      (:A
        (Variables|/Script/Engine.PlayerController|SetbShowMouseCursor _returnvalue true)
        (Input|SetInputModeGameandUI _returnvalue_2 0 "DoNotLock" true false))
      (:B
        (Variables|/Script/Engine.PlayerController|SetbShowMouseCursor _returnvalue false)
        (Input|SetInputModeGameOnly _returnvalue_2 false)))))

(event Input|KeyboardEvents|1
  (params (Key :type Key%20Structure :default "None"))
  (:Pressed
    (Utilities|SetViewMode 1.0
      (:then
        (Variables|Default|SetViewMode "NewEnumerator1")))))

(event Input|KeyboardEvents|4
  (params (Key :type Key%20Structure :default "None"))
  (:Pressed
    (Utilities|SetViewMode 4.0
      (:then
        (Variables|Default|SetViewMode "NewEnumerator4")))))

(event Input|KeyboardEvents|2
  (params (Key :type Key%20Structure :default "None"))
  (:Pressed
    (Utilities|SetViewMode 2.0
      (:then
        (Variables|Default|SetViewMode "NewEnumerator2")))))

(event Input|KeyboardEvents|3
  (params (Key :type Key%20Structure :default "None"))
  (:Pressed
    (Utilities|SetViewMode 3.0
      (:then
        (Variables|Default|SetViewMode "NewEnumerator3")))))

(fn ConstructionScript)