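; BP_FlipBookOverView is a showcase actor that previews a flipbook effect in Niagara with a text label.
; Its Construction Script passes the material, DTFA and MVN textures, hue, color and lifetime into the Niagara component as user variables.
; It sets the TextRender label through GetName on the DTFA texture, whose graph holds an unconnected underscore-split of the asset's display name.
; All event graph events are empty.
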(event EventBeginPlay)

(event Collision|EventActorBeginOverlap
  (params (OtherActor :type Actor%20Object%20Reference)))

(event EventTick
  (params (DeltaSeconds :type Float%20%28single-precision%29)))

(fn ConstructionScript
  (Rendering|Components|TextRender|SetText (Variables|Default|GetTextRender) (|GetName (Variables|Default|GetDTFA)))
  (Class|NiagaraComponent|SetVariableMaterial (Variables|Default|GetNiagara) "Mat" (Variables|Default|GetMat))
  (Class|NiagaraComponent|SetVariableTexture (Variables|Default|GetNiagara) "DTFA" (Variables|Default|GetDTFA))
  (Class|NiagaraComponent|SetVariableTexture (Variables|Default|GetNiagara) "MVN" (Variables|Default|GetMVN))
  (Niagara|SetNiagaraVariable(Float) (Variables|Default|GetNiagara) "Hue" (Variables|Default|GetHue))
  (Niagara|SetNiagaraVariable(LinearColor) (Variables|Default|GetNiagara) "Color" (Variables|Default|GetColor))
  (Niagara|SetNiagaraVariable(Float) (Variables|Default|GetNiagara) "LifeTime" (Variables|Default|GetLifeTime)))